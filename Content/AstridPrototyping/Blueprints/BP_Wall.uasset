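; BP_Wall is a prototyping actor that builds a straight wall from repeated mesh segments.
; Its construction script loops over WallLength, adding a static mesh component for each segment at a multiple of SegmentLength along local X.
; Each segment uses WallMesh with a shared ZRotation yaw and writes to custom depth with a fixed stencil value.
; The event graph has no active logic.
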(fn `CalculateXLocation`
  (params (Index :type Integer))
  (returns (XLocation :type "Float (double-precision)"))
  (return (* (- Index 1) (`self.SegmentLength`))))

(fn `CreateMesh`
  (params (XLocation :type "Float (double-precision)"))
  (bind _returnvalue (`AddComponent|NODE_AddStaticMeshComponent-0`))
  (`PrimitiveComponent.SetRenderCustomDepth` _returnvalue true)
  (`PrimitiveComponent.SetCustomDepthStencilValue` _returnvalue 5)
  (`StaticMeshComponent.SetStaticMesh` _returnvalue (`self.WallMesh`))
  (`SceneComponent.K2_SetRelativeLocationAndRotation` _returnvalue (`KismetMathLibrary.MakeVector` XLocation) (`KismetMathLibrary.MakeRotator` 0.0 0.0 (`self.ZRotation`)) false false))

(fn `UserConstructionScript`
  (for _index (range 1 (+ (`self.WallLength`) 1))
    (`self.CreateMesh` (`self.CalculateXLocation` _index))))