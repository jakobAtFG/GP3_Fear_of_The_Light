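; BP_AlphaMainMenu is a prototype main menu Blueprint that runs the opening sequence of the alpha menu.
; On BeginPlay it starts a camera fade from black and waits out the fade duration before showing the WBP_AdjustVisibility widget.
; It then disables player character input, shows the mouse cursor and switches to UI-only input focused on that widget.
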(event `self.ReceiveBeginPlay`
  (bind _returnvalue (`GameplayStatics.GetPlayerController` 0))
  (`PlayerCameraManager.StartCameraFade` (`GameplayStatics.GetPlayerCameraManager` 0) 1.0 0.0 (`self.StartFadeDuration`) (struct :`A` 1.0) false false)
  (`KismetSystemLibrary.Delay` (`self.StartFadeDuration`))
  (bind _returnvalue_2 (`|CreateWidget` "/Game/WBP/WBP_AdjustVisibility.WBP_AdjustVisibility_C"))
  (`UserWidget.AddToViewport` _returnvalue_2 0)
  (`self.DisableInput` (`GameplayStatics.GetPlayerCharacter` 0) _returnvalue)
  (set `PlayerController.bShowMouseCursor` true _returnvalue)
  (`WidgetBlueprintLibrary.SetInputMode_UIOnlyEx` _returnvalue _returnvalue_2))

(fn `UserConstructionScript`)