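; Prototype proximity charger that raises or drains the battery of the level's BP_PROT_BatterySystem while the player character stands inside its sphere.
; BeginPlay finds the battery system, sets the tick interval from ChargeTick and hides the point light.
; Sphere overlaps toggle the Charging flag and the light.
; While Charging, each tick adds IncreaseAmount until full, or subtracts it when IsAdditive is off.
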(event `self.ReceiveBeginPlay`
  (bind _returnvalue (`GameplayStatics.GetActorOfClass` "/Game/AstridPrototyping/Blueprints/BP_PROT_BatterySystem.BP_PROT_BatterySystem_C"))
  (`/Engine/EditorBlueprintResources/StandardMacros.IsValid` _returnvalue
    (:`Is Valid`
      (set `self.BatterySystem` _returnvalue)
      ;[1 1 1] Setting Tick... god help us all
      (`self.SetActorTickInterval` (`self.ChargeTick`))
      (`SceneComponent.SetVisibility` (`self.PointLight`) false false))))

(event `self.ReceiveTick`
  (params (DeltaSeconds :type "Float (single-precision)"))
  (if (`self.Charging`)
    (if (`self.IsAdditive`)
      (if (not (`/Game/AstridPrototyping/Blueprints/BP_PROT_BatterySystem.IsBatteryFull` (`self.BatterySystem`)))
        (`/Game/AstridPrototyping/Blueprints/BP_PROT_BatterySystem.IncreaseBatteryPercent` (`self.BatterySystem`) (`self.IncreaseAmount`)))
      (else
        (`/Game/AstridPrototyping/Blueprints/BP_PROT_BatterySystem.DecreaseBatteryPercent` (`self.BatterySystem`) (`self.IncreaseAmount`))))))

(event `self.Sphere.OnComponentBeginOverlap`
  (params (OverlappedComponent :type "PrimitiveComponent Object Reference") (OtherActor :type "Actor Object Reference") (OtherComp :type "PrimitiveComponent Object Reference") (OtherBodyIndex :type Integer) (bFromSweep :type Boolean) (SweepResult :type "HitResult Structure (by ref)"))
  (if (== OtherActor (`GameplayStatics.GetPlayerCharacter` 0))
    (set `self.Charging` true)
    (`SceneComponent.SetVisibility` (`self.PointLight`) true false)))

(event `self.Sphere.OnComponentEndOverlap`
  (params (OverlappedComponent :type "PrimitiveComponent Object Reference") (OtherActor :type "Actor Object Reference") (OtherComp :type "PrimitiveComponent Object Reference") (OtherBodyIndex :type Integer))
  (if (== OtherActor (`GameplayStatics.GetPlayerCharacter` 0))
    (set `self.Charging` false)
    (`SceneComponent.SetVisibility` (`self.PointLight`) false false)))

(fn `UserConstructionScript`)