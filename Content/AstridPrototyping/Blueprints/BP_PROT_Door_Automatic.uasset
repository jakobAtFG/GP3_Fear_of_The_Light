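; Automatic sliding door that opens for overlapping Pawns while unlocked and closes once the last one leaves.
; A timeline moves the upper and lower panels, and ToggleDoor plays audio and delays disabling collision when opening.
; OnInteract sets or toggles the lock, optionally once, updating frame materials and holo-text signage and rechecking overlaps.
; Unlocked state persists through GameManager save events, keyed by the door's display name.
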(event `AnimateDoor`
  (`SceneComponent.SetVisibility` (`self.HoloTextActor`) false true)
  (bind (_direction _door_upper _door_lower) (`Timeline|DoorTimeline` :!via `PlayFromStart` :!label _label)
    (:`Update`
      (`SceneComponent.K2_SetRelativeLocation` (`self.DoorPlaneUpper`) _door_upper false false)
      (`SceneComponent.K2_SetRelativeLocation` (`self.DoorPlaneLower`) _door_lower false false))
    (:`Finished`
      (switch `ETimelineDirection` _direction
        (:`Backward`
          (`SceneComponent.SetVisibility` (`self.HoloTextActor`) true true))))))

(event `ReverseAnimateDoor`
  (goto _label :!via `ReverseFromEnd`))

(event `self.Collider.OnComponentBeginOverlap`
  (params (OverlappedComponent :type "PrimitiveComponent Object Reference") (OtherActor :type "Actor Object Reference") (OtherComp :type "PrimitiveComponent Object Reference") (OtherBodyIndex :type Integer) (bFromSweep :type Boolean) (SweepResult :type "HitResult Structure (by ref)"))
  (bind _overlappingactors (`self.OverlappingActors`))
  (if (`self.Unlocked`)
    (cast `Pawn` OtherActor)
    (if (> (`KismetArrayLibrary.Array_Length` _overlappingactors) 0)
      (if (not (`KismetArrayLibrary.Array_Contains` _overlappingactors OtherActor))
        (`KismetArrayLibrary.Array_AddUnique` _overlappingactors OtherActor :!label _label_2)
        (if (not (`self.DoorOpen`))
          (`self.ToggleDoor` true)))
      (else
        (goto _label_2)))))

(event `self.Collider.OnComponentEndOverlap`
  (params (OverlappedComponent :type "PrimitiveComponent Object Reference") (OtherActor :type "Actor Object Reference") (OtherComp :type "PrimitiveComponent Object Reference") (OtherBodyIndex :type Integer))
  (bind _overlappingactors (`self.OverlappingActors`))
  (bind _returnvalue (> (`KismetArrayLibrary.Array_Length` _overlappingactors) 0))
  (if (`self.Unlocked`)
    (cast `Pawn` OtherActor)
    (if _returnvalue
      (if (`KismetArrayLibrary.Array_Contains` _overlappingactors OtherActor)
        (`KismetArrayLibrary.Array_RemoveItem` _overlappingactors OtherActor)
        (if (and (`self.DoorOpen`) (not _returnvalue))
          (`self.ToggleDoor` false))))))

(event `self.OnInteract`
  (params (bIsActive :type Boolean) (InteractionType :type "/Game/BP/E_InteractionType Enum" :default "NewEnumerator0"))
  (bind _unlocked (`self.Unlocked`))
  (if (`self.OnlyInteractOnce`)
    (if (not (`self.Interacted`))
      (set `self.Interacted` true :!label _label_3)
      (switch `/Game/BP/E_InteractionType` InteractionType
        (:`NewEnumerator0`
          (if bIsActive
            (set `self.Unlocked` true :!label _label_4)
            (else
              (set `self.Unlocked` false :!label _label_5))))
        (:`NewEnumerator2`
          (if _unlocked
            (goto _label_5)
            (else
              (goto _label_4)))))
      (`self.UpdateVisualsOnUnlocked` _unlocked)
      (if (`self.Unlocked`)
        (`self.CheckForOverlappingActors`)))
    (else
      (goto _label_3))))

(event `DisableDoorCollision`
  ;[1 1 1] So that you can't walk through the door until it's fully open
  (`KismetSystemLibrary.Delay` 0.25)
  (`PrimitiveComponent.SetCollisionEnabled` (`self.DoorCollider`) "NoCollision"))

(event `self.ReceiveBeginPlay`
  (bind _asgame_manager (cast `GameManager` (`GameplayStatics.GetGameInstance`)))
  (`|ExecutionSequence`
    (:`then_0`
      (add `GameManager.OnSaveRequested` _asgame_manager (delegate `OnSaveRequested_Event`)))
    (:`then_1`
      (add `GameManager.OnSaveDataLoaded` _asgame_manager (delegate `OnSaveDataLoaded_Event`)))
    (:`then_2`
      (`KismetSystemLibrary.DelayUntilNextTick`)
      (`self.CheckForOverlappingActors`))))

(event `OnSaveRequested_Event`
  (params (SaveGame :type "GP3SaveGame Object Reference"))
  (if (`self.Unlocked`)
    (`KismetArrayLibrary.Array_AddUnique` (`GP3SaveGame.UnlockedDoors` SaveGame) (`KismetSystemLibrary.GetDisplayName` self))))

(event `OnSaveDataLoaded_Event`
  (params (SaveGame :type "GP3SaveGame Object Reference"))
  (if (`KismetArrayLibrary.Array_Contains` (`GP3SaveGame.UnlockedDoors` SaveGame) (`KismetSystemLibrary.GetDisplayName` self))
    (bind _output_get (set `self.Unlocked` true))
    (`self.UpdateVisualsOnUnlocked` _output_get)
    (else
      (bind _output_get_2 (set `self.Unlocked` false))
      (`self.UpdateVisualsOnUnlocked` _output_get_2))))

(fn `CheckForOverlappingActors`
  (bind _overlappingactors (`self.OverlappingActors`))
  (bind _overlappingactors_2 (`PrimitiveComponent.GetOverlappingActors` (`self.Collider`) "/Script/Engine.Pawn"))
  (if (`self.Unlocked`)
    (if (> (`KismetArrayLibrary.Array_Length` _overlappingactors_2) 0)
      (for _array_element _overlappingactors_2
        (if (> (`KismetArrayLibrary.Array_Length` _overlappingactors) 0)
          (if (not (`KismetArrayLibrary.Array_Contains` _overlappingactors _array_element))
            (`KismetArrayLibrary.Array_AddUnique` _overlappingactors _array_element :!label _label))
          (else
            (goto _label))))
      (if (not (`self.DoorOpen`))
        (`self.ToggleDoor` true)))))

(fn `ToggleDoor`
  (params (NewActive :type Boolean))
  (if NewActive
    (`self.AnimateDoor`)
    (`AudioComponent.Play` (`self.Audio`) 0.0)
    (set `self.DoorOpen` true)
    (`self.DisableDoorCollision`)
    (else
      (`self.ReverseAnimateDoor`)
      (`PrimitiveComponent.SetCollisionEnabled` (`self.DoorCollider`) "QueryAndPhysics")
      (`AudioComponent.Play` (`self.Audio`) 0.0)
      (set `self.DoorOpen` false))))

(fn `UpdateVisualsOnUnlocked`
  (params (Unlocked :type Boolean))
  (bind _door_frame (`self.Door_Frame`))
  (bind _lockedmaterial (`self.LockedMaterial`))
  (bind _door_frame_2 (`self.Door_Frame`))
  (bind _returnvalue (`KismetTextLibrary.TextToUpper` (`self.ClearanceLevelText`)))
  (bind _returnvalue_2 (`KismetMathLibrary.Conv_LinearColorToColor` (`KismetMathLibrary.MakeColor` 1.0)))
  (bind _returnvalue_3 (`KismetMathLibrary.Conv_LinearColorToColor` (`KismetMathLibrary.MakeColor` 1.0 0.913796 0.316616)))
  (if Unlocked
    (`PrimitiveComponent.SetMaterial` _door_frame 1 (`self.DefaultMaterial`))
    (`PrimitiveComponent.SetMaterial` _door_frame 2 (`self.DefaultMaterial`))
    (`SceneComponent.SetVisibility` (`self.RollingText`) false true)
    (bind _asbp_holo_text (cast `/Game/BP/BP_HoloText` (`ChildActorComponent.ChildActor` (`self.HoloTextActor`))))
    (`/Game/BP/BP_HoloText.SetTextAndColor` _asbp_holo_text "UNLOCKED" _returnvalue_3)
    (bind _asbp_holo_text_2 (cast `/Game/BP/BP_HoloText` (`ChildActorComponent.ChildActor` (`self.HoloTextActor1`))))
    (`/Game/BP/BP_HoloText.SetTextAndColor` _asbp_holo_text_2 "UNLOCKED" _returnvalue_3)
    (else
      (`PrimitiveComponent.SetMaterial` _door_frame_2 1 _lockedmaterial)
      (`PrimitiveComponent.SetMaterial` _door_frame_2 2 _lockedmaterial)
      (`SceneComponent.SetVisibility` (`self.RollingText`) true true)
      (bind _asbp_holo_text_3 (cast `/Game/BP/BP_HoloText` (`ChildActorComponent.ChildActor` (`self.HoloTextActor`))))
      (`/Game/BP/BP_HoloText.SetTextAndColor` _asbp_holo_text_3 _returnvalue _returnvalue_2)
      (bind _asbp_holo_text_4 (cast `/Game/BP/BP_HoloText` (`ChildActorComponent.ChildActor` (`self.HoloTextActor1`))))
      (`/Game/BP/BP_HoloText.SetTextAndColor` _asbp_holo_text_4 _returnvalue _returnvalue_2))))

(fn `UserConstructionScript`
  (bind _returnvalue (`KismetMathLibrary.Conv_LinearColorToColor` (`KismetMathLibrary.MakeColor` 1.0 0.913796 0.316616)))
  (bind _asbp_holo_text (cast `/Game/BP/BP_HoloText` (`ChildActorComponent.ChildActor` (`self.HoloTextActor2`))))
  (`/Game/BP/BP_HoloText.SetTextAndColor` _asbp_holo_text (`KismetTextLibrary.TextToUpper` (`self.DoorNameFront`)) _returnvalue)
  (bind _asbp_holo_text_2 (cast `/Game/BP/BP_HoloText` (`ChildActorComponent.ChildActor` (`self.HoloTextActor3`))))
  (`/Game/BP/BP_HoloText.SetTextAndColor` _asbp_holo_text_2 (`KismetTextLibrary.TextToUpper` (`self.DoorNameBack`)) _returnvalue)
  (`self.UpdateVisualsOnUnlocked` (`self.Unlocked`)))