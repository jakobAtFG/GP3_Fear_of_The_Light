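; Prototype shutter door that opens and closes through an interact event, starting in a configurable state.
; OnInteract supports Control and Toggle modes, optionally only once, and calls ToggleDoor.
; ToggleDoor plays animation and audio, switches collision and forwards state to optional HoloText; both directions play the Close animation.
; Older battery-cost and proximity logic is disconnected, and the collision-disable delay is zero.
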(event `self.ReceiveBeginPlay`
  (if (`self.DoorOpenAtStart`)
    (`self.ToggleDoor` true)
    (else
      (`self.ToggleDoor` false)))
  (set `self.Interacted` false))

(event `self.Collider.OnComponentBeginOverlap`
  (params (OverlappedComponent :type "PrimitiveComponent Object Reference") (OtherActor :type "Actor Object Reference") (OtherComp :type "PrimitiveComponent Object Reference") (OtherBodyIndex :type Integer) (bFromSweep :type Boolean) (SweepResult :type "HitResult Structure (by ref)"))
  ;[1 1 1] Deprecated
)

(event `self.Collider.OnComponentEndOverlap`
  (params (OverlappedComponent :type "PrimitiveComponent Object Reference") (OtherActor :type "Actor Object Reference") (OtherComp :type "PrimitiveComponent Object Reference") (OtherBodyIndex :type Integer))
  ;[1 1 1] Deprecated
)

(event `Key|F`
  (params (Key :type "Key Structure"))
  ;[1 1 1] Deprecated
)

(event `/Game/BP/BI_Interactable.OnInteract`
  (params (bIsActive :type Boolean) (InteractionType :type "/Game/BP/E_InteractionType Enum" :default "NewEnumerator0"))
  (if (`self.OnlyInteractOnce`)
    (if (not (`self.Interacted`))
      (switch `/Game/BP/E_InteractionType` InteractionType :!label _label
        (:`NewEnumerator0`
          (if bIsActive
            (`self.ToggleDoor` true :!label _label_2)
            (else
              (`self.ToggleDoor` false :!label _label_3))))
        (:`NewEnumerator2`
          (if (`self.DoorOpen`)
            (goto _label_3)
            (else
              (goto _label_2)))))
      (set `self.Interacted` true))
    (else
      (goto _label))))

(event `DisableDoorCollision`
  ;[1 1 1] So that you can't walk through the door until it's fully open
  (`KismetSystemLibrary.Delay` 0.0)
  (`PrimitiveComponent.SetCollisionEnabled` (`self.DoorCollider`) "NoCollision"))

(fn `ToggleDoor`
  (params (NewActive :type Boolean))
  (bind _holotext (`self.HoloText`))
  (bind _holotext_2 (`self.HoloText`))
  (bind _doorskeleton (`self.DoorSkeleton`))
  (bind _doorskeleton_2 (`self.DoorSkeleton`))
  (if NewActive
    (`SkeletalMeshComponent.Stop` _doorskeleton_2)
    (`SkeletalMeshComponent.PlayAnimation` _doorskeleton_2 "/Game/Art/3D/Enviorment/Doors/Door_Shutter_Anim_Close.Door_Shutter_Anim_Close" false)
    (`AudioComponent.Play` (`self.Audio`) 0.0)
    (set `self.DoorOpen` true)
    (`self.DisableDoorCollision`)
    (`/Engine/EditorBlueprintResources/StandardMacros.IsValid` _holotext_2
      (:`Is Valid`
        (message `/Game/BP/BI_Interactable.OnInteract` _holotext_2 true "NewEnumerator0")))
    (else
      (`SkeletalMeshComponent.Stop` _doorskeleton)
      (`SkeletalMeshComponent.PlayAnimation` _doorskeleton "/Game/Art/3D/Enviorment/Doors/Door_Shutter_Anim_Close.Door_Shutter_Anim_Close" false)
      (`PrimitiveComponent.SetCollisionEnabled` (`self.DoorCollider`) "QueryAndPhysics")
      (`AudioComponent.Play` (`self.Audio`) 0.0)
      (set `self.DoorOpen` false)
      (`/Engine/EditorBlueprintResources/StandardMacros.IsValid` _holotext
        (:`Is Valid`
          (message `/Game/BP/BI_Interactable.OnInteract` _holotext false "NewEnumerator0"))))))

(fn `UserConstructionScript`)