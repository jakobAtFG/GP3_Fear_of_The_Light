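; Interactable data terminal with an in-world screen widget, tagged as radar-detectable.
; Interacting unequips the tool and toggles use, blending the view, switching input and swapping info and controls widgets.
; BeginPlay initializes the screen with tab, log and item data, binding close and map events; map events toggle control hints.
; GameManager save events record overrides by display name, but loading checks for an empty string before disabling the override.
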(event `self.ReceiveBeginPlay`
  (`parent.ReceiveBeginPlay`)
  (`|ExecutionSequence`
    (:`then_0`
      (set `self.IsActive` false)
      (bind _aswbp_data_terminal (cast `/Game/WBP/WBP_DataTerminal` (`WidgetComponent.GetWidget` (`self.Widget`))))
      (bind _output_get (set `self.WidgetDataTerminal` _aswbp_data_terminal))
      (`/Game/WBP/WBP_DataTerminal.Initialize` _output_get (`self.Show Map Tab`) (`self.System Item Array`) (`self.AreaItem`) (`self.TerminalIndex`) (`self.LogArray`))
      (add `/Game/WBP/WBP_DataTerminal.OnCloseClicked` (`self.WidgetDataTerminal`) (`|CreateDelegate` :!event `InteractEventFunction`))
      (add `/Game/WBP/WBP_DataTerminal.OnMapOpened` (`self.WidgetDataTerminal`) (`|CreateDelegate` :!event `MapOpened`))
      (add `/Game/WBP/WBP_DataTerminal.OnMapClosed` (`self.WidgetDataTerminal`) (`|CreateDelegate` :!event `MapClosed`)))
    (:`then_1`
      (bind _asgame_manager (cast `GameManager` (`GameplayStatics.GetGameInstance`)))
      (`|ExecutionSequence`
        (:`then_0`
          (add `GameManager.OnSaveRequested` _asgame_manager (delegate `OnSaveRequested_Event`)))
        (:`then_1`
          (add `GameManager.OnSaveDataLoaded` _asgame_manager (delegate `OnSaveDataLoaded_Event`)))))))

(event `OnSaveRequested_Event`
  (params (SaveGame :type "GP3SaveGame Object Reference"))
  (if (`/Game/WBP/WBP_DataTerminal.GetOverrideStatus` (`self.WidgetDataTerminal`))
    (`KismetArrayLibrary.Array_AddUnique` (`GP3SaveGame.TerminalOverrides` SaveGame) (`KismetSystemLibrary.GetDisplayName` self))))

(event `OnSaveDataLoaded_Event`
  (params (SaveGame :type "GP3SaveGame Object Reference"))
  (bind _widgetdataterminal (`self.WidgetDataTerminal`))
  (if (`KismetArrayLibrary.Array_Contains` (`GP3SaveGame.TerminalOverrides` SaveGame))
    (`KismetSystemLibrary.DelayUntilNextTick`)
    (`/Engine/EditorBlueprintResources/StandardMacros.IsValid` _widgetdataterminal
      (:`Is Valid`
        (`/Game/WBP/WBP_DataTerminal.DisableOverride` _widgetdataterminal)))))

(fn `GetGameplayTags`
  (returns (GameplayTagContainer :type "GameplayTagContainer Structure"))
  (return (struct :`GameplayTags` (struct :`(TagName` "RadarDetectable.DataTerminal")))))

(fn `InteractEventFunction`
  (bind _returnvalue (`GameplayStatics.GetPlayerController` 0))
  (`parent.InteractEventFunction`)
  (`ToolManager.UnequipTool` (`self.GetComponentByClass` (`GameplayStatics.GetPlayerPawn` 0) "/Script/GP3.ToolManager"))
  (if (`self.IsActive`)
    (set `PlayerController.bShowMouseCursor` false _returnvalue)
    (`PlayerController.SetViewTargetWithBlend` _returnvalue (`GameplayStatics.GetPlayerCharacter` 0) 0.5 "VTBlend_Linear" 0.0 false)
    (`Controller.SetIgnoreMoveInput` _returnvalue false)
    (set `self.IsActive` false)
    (`WidgetBlueprintLibrary.SetInputMode_GameOnly` (`GameplayStatics.GetPlayerController` 0))
    (`self.Show Info Widget`)
    (`/Game/WBP/WBP_DataTerminal.SetupSignIn` (`self.WidgetDataTerminal`))
    (`GameplayStatics.PlaySoundAtLocation` "/Game/Audio/Terminal/SFX_DATA_BEEP.SFX_DATA_BEEP" (`self.K2_GetActorLocation` self) (struct) 1.0 1.0 0.0 null null null null)
    (`Widget.RemoveFromParent` (`self.WidgetControls`))
    (set `self.WidgetControls` null)
    (else
      (set `PlayerController.bShowMouseCursor` true _returnvalue)
      (`PlayerController.SetViewTargetWithBlend` _returnvalue self 0.5 "VTBlend_Linear" 0.0 false)
      (`Controller.SetIgnoreMoveInput` _returnvalue true)
      (set `self.IsActive` true)
      (`WidgetBlueprintLibrary.SetInputMode_GameAndUIEx` (`GameplayStatics.GetPlayerController` 0) (`WidgetComponent.GetWidget` (`self.Widget`)))
      (`self.Close Info Widget`)
      (`GameplayStatics.PlaySoundAtLocation` "/Game/Audio/Terminal/SFX_DATA_USE.SFX_DATA_USE" (`self.K2_GetActorLocation` self) (struct) 1.0 1.0 0.0 null null null null)
      (bind _returnvalue_2 (`|CreateWidget` "/Game/WBP/WBP_DataTerminalControls.WBP_DataTerminalControls_C"))
      (bind _output_get (set `self.WidgetControls` _returnvalue_2))
      (`UserWidget.AddToViewport` _output_get 0))))

(fn `MapClosed`
  (`/Engine/EditorBlueprintResources/StandardMacros.IsValid` (`self.WidgetControls`)
    (:`Is Valid`
      (`/Game/WBP/WBP_DataTerminalControls.ShowMapControls` (`self.WidgetControls`) false))))

(fn `MapOpened`
  (`/Engine/EditorBlueprintResources/StandardMacros.IsValid` (`self.WidgetControls`)
    (:`Is Valid`
      (`/Game/WBP/WBP_DataTerminalControls.ShowMapControls` (`self.WidgetControls`) true))))

(fn `UserConstructionScript`
  (`parent.UserConstructionScript`))