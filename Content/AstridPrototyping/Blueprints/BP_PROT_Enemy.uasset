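; Prototype moth enemy that chases the player on entering its detection sphere and triggers a paused game-over screen when its attack sphere overlaps them.
; AI MoveTo drives the chase while particle intensity and audio pitch and volume rise.
; Tick drops the chase beyond ChaseRange, resetting effects and returning it to its start point, or to a cached light position once NewLightEnabled has fired.
; The construction script sizes both spheres from radius variables.
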(event `self.ReceiveBeginPlay`
  (set `self.StartLocation` (`self.K2_GetActorLocation`))
  (set `self.LightPoint` (`self.K2_GetActorLocation` (`self.LightPointActor`))))

(event `self.ReceiveTick`
  (params (DeltaSeconds :type "Float (single-precision)"))
  (if (`self.Chasing`)
    (if (> (`self.GetDistanceTo` (`GameplayStatics.GetPlayerCharacter` 0) self) (`self.ChaseRange`))
      (set `self.Chasing` false)
      (set `self.Returning` true)
      (`NiagaraComponent.SetVariableFloat` (`self.FXS_MothPrototype`) "Intensity" 4.0)
      (`AudioComponent.SetPitchMultiplier` (`self.Audio`) 1.0)
      (`AudioComponent.SetVolumeMultiplier` (`self.Audio`) 1.0))
    (elif (`self.Returning`)
      (if (`self.LightOn`)
        (`|AIMoveTo` self (`self.LightPoint`) null
          (:`then`
            (set `self.Returning` false)))
        (else
          (`|AIMoveTo` self (`self.StartLocation`) null
            (:`then`
              (set `self.Returning` false))))))))

(event `NewLightEnabled`
  (set `self.LightOn` true)
  (set `self.Returning` true))

(event `self.MurderCollider.OnComponentBeginOverlap`
  (params (OverlappedComponent :type "PrimitiveComponent Object Reference") (OtherActor :type "Actor Object Reference") (OtherComp :type "PrimitiveComponent Object Reference") (OtherBodyIndex :type Integer) (bFromSweep :type Boolean) (SweepResult :type "HitResult Structure (by ref)"))
  ;[1 1 1] Scuffed kill
  (if (== OtherActor (`GameplayStatics.GetPlayerCharacter` 0))
    (`self.GameOver`)))

(event `self.DetectPlayerCollider.OnComponentBeginOverlap`
  (params (OverlappedComponent :type "PrimitiveComponent Object Reference") (OtherActor :type "Actor Object Reference") (OtherComp :type "PrimitiveComponent Object Reference") (OtherBodyIndex :type Integer) (bFromSweep :type Boolean) (SweepResult :type "HitResult Structure (by ref)"))
  (bind _returnvalue (`GameplayStatics.GetPlayerCharacter` 0))
  ;[1 1 1] Scuffed Chase the player when they get close in range...
  (if (== OtherActor _returnvalue)
    (if (not (`self.Chasing`))
      (`|AIMoveTo` self (0.0 0.0 0.0) _returnvalue
        (:`then`
          (set `self.Chasing` true)
          (`NiagaraComponent.SetVariableFloat` (`self.FXS_MothPrototype`) "Intensity" 20.0)
          (`AudioComponent.SetPitchMultiplier` (`self.Audio`) 2.0)
          (`AudioComponent.SetVolumeMultiplier` (`self.Audio`) 2.0))))))

(fn `GameOver`
  (bind _returnvalue (`|CreateWidget` "/Game/WBP/WBP_GameOver_PROT.WBP_GameOver_PROT_C"))
  (`UserWidget.AddToViewport` _returnvalue 0)
  (`GameplayStatics.SetGamePaused` true)
  (set `PlayerController.bShowMouseCursor` true (`GameplayStatics.GetPlayerController` 0)))

(fn `UserConstructionScript`
  (`SphereComponent.SetSphereRadius` (`self.DetectPlayerCollider`) (`self.DetectRadius`) true)
  (`SphereComponent.SetSphereRadius` (`self.MurderCollider`) (`self.AttackRadius`) true))