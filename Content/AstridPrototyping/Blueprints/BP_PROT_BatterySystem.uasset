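; Prototype battery system Blueprint that tracks a charge level as a normalized percentage and shows it on a HUD.
; On BeginPlay it creates the WBP_BatteryHUD widget, adds it to the viewport and sets the starting value.
; Increase and decrease functions clamp the charge between empty and full, then push it to the widget.
; Query functions report whether the battery is full or holds enough charge for a given amount.
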(event `self.ReceiveBeginPlay`
  ;[1 1 1] Add UI
  (bind _returnvalue (`|CreateWidget` "/Game/WBP/WBP_BatteryHUD.WBP_BatteryHUD_C" null (`self.BatteryPercent`)))
  (bind _output_get (set `self.BatteryWidget` _returnvalue))
  (`/Game/WBP/WBP_BatteryHUD.SetPercent` _output_get (`self.BatteryPercent`))
  (`UserWidget.AddToViewport` (`self.BatteryWidget`) 0))

(fn `DecreaseBatteryPercent`
  (params (Percent :type "Float (double-precision)"))
  (set `self.BatteryPercent` (`KismetMathLibrary.FClamp` (- (`self.BatteryPercent`) Percent)))
  (`self.UpdateUI`))

(fn `HasEnoughBattery`
  (params (Percent :type "Float (double-precision)"))
  (returns (HasEnoughBattery :type Boolean))
  (return (>= (`self.BatteryPercent`) Percent)))

(fn `IncreaseBatteryPercent`
  (params (Percent :type "Float (double-precision)"))
  (set `self.BatteryPercent` (`KismetMathLibrary.FClamp` (+ Percent (`self.BatteryPercent`))))
  (`self.UpdateUI`))

(fn `IsBatteryFull`
  (returns (IsBatteryFull :type Boolean))
  (return (== (`self.BatteryPercent`) 1.0)))

(fn `UpdateUI`
  (`/Game/WBP/WBP_BatteryHUD.SetPercent` (`self.BatteryWidget`) (`self.BatteryPercent`)))

(fn `UserConstructionScript`)