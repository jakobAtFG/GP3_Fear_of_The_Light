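; Procedural corridor actor that builds two facing rows of wall segments in its Construction Script.
; Two loops over RowLength call CreateWall, placing WallMesh components at SegmentLength intervals on either side at RowWidth, with one row yawed 180 degrees.
; Each segment writes to custom depth with a fixed stencil value.
; The event graph is empty, and a disconnected block for positioning and stretching thin elements along both sides never runs.
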(fn `CreateWall`
  (params (Index :type Integer) (YLocation :type "Float (double-precision)") (ZRotation :type "Float (double-precision)"))
  (bind _returnvalue (`AddComponent|NODE_AddStaticMeshComponent-0`))
  (`StaticMeshComponent.SetStaticMesh` _returnvalue (`self.WallMesh`))
  (`SceneComponent.K2_SetRelativeLocationAndRotation` _returnvalue (`KismetMathLibrary.MakeVector` (* (- Index 1) (`self.SegmentLength`)) YLocation) (`KismetMathLibrary.MakeRotator` 0.0 0.0 ZRotation) false false)
  (`PrimitiveComponent.SetRenderCustomDepth` _returnvalue true)
  (`PrimitiveComponent.SetCustomDepthStencilValue` _returnvalue 5))

(fn `UserConstructionScript`
  (bind _rowwidth (`self.RowWidth`))
  (`|ExecutionSequence`
    (:`then_0`
      (for _index (range 1 (+ (`self.RowLength`) 1))
        (`self.CreateWall` _index (- _rowwidth (* _rowwidth 2.0)))))
    (:`then_1`
      (for _index_2 (range 1 (+ (`self.RowLength`) 1))
        (`self.CreateWall` _index_2 (`self.RowWidth`) 180.0)))))