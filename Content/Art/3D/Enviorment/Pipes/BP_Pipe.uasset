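; BP_Pipe is an environment actor that builds a pipe along a spline from a repeated static mesh.
; The construction script derives segment length from the mesh bounds on the chosen forward axis and XScale, then adds spline mesh components along the spline.
; Tangents are clamped to segment length, and XOffset shifts each segment's end.
; Segments write custom depth stencil, and EnableCollision works inverted: true disables collision.
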(event `self.ReceiveTick`
  (params (DeltaSeconds :type "Float (single-precision)")))

(fn `UserConstructionScript`
  (bind _spline (`self.Spline`))
  (bind _spline_2 (`self.Spline`))
  (bind (_returnvalue_min _returnvalue_max) (break `Box` (`StaticMesh.GetBoundingBox` (`self.Mesh`))))
  (bind (_returnvalue_x _returnvalue_y _returnvalue_z) (`KismetMathLibrary.BreakVector` (* (- _returnvalue_max _returnvalue_min) (`self.XScale`))))
  (switch `ESplineMeshAxis` (`self.ForwardAxis`)
    (:`X`
      (set `self.XLength` _returnvalue_x))
    (:`Y`
      (set `self.XLength` _returnvalue_y))
    (:`Z`
      (set `self.XLength` _returnvalue_z)))
  (for _index (range (+ (`KismetMathLibrary.FTrunc` (/ (`SplineComponent.GetSplineLength` (`self.Spline`)) (`self.XLength`))) 1))
    (bind _returnvalue (`AddComponent|NODE_AddSplineMeshComponent-0`))
    (`PrimitiveComponent.SetRenderCustomDepth` _returnvalue true)
    (`PrimitiveComponent.SetCustomDepthStencilValue` _returnvalue 5)
    (if (`self.EnableCollision`)
      (`PrimitiveComponent.SetCollisionEnabled` _returnvalue "NoCollision")
      (else
        (`PrimitiveComponent.SetCollisionEnabled` _returnvalue "QueryAndPhysics")))
    (`SplineMeshComponent.SetForwardAxis` _returnvalue (`self.ForwardAxis`) true)
    (`StaticMeshComponent.SetStaticMesh` _returnvalue (`self.Mesh`))
    (bind _returnvalue_2 (* _index (`self.XLength`)))
    (bind _returnvalue_3 (* (+ (+ _index 1) (`self.XOffset`)) (`self.XLength`)))
    (`SplineMeshComponent.SetStartAndEnd` _returnvalue (`SplineComponent.GetLocationAtDistanceAlongSpline` _spline_2 _returnvalue_2 "Local") (`KismetMathLibrary.ClampVectorSize` (`SplineComponent.GetTangentAtDistanceAlongSpline` _spline_2 _returnvalue_2 "Local") 0.0 (`self.XLength`)) (`SplineComponent.GetLocationAtDistanceAlongSpline` _spline _returnvalue_3 "Local") (`KismetMathLibrary.ClampVectorSize` (`SplineComponent.GetTangentAtDistanceAlongSpline` _spline _returnvalue_3 "Local") 0.0 (`self.XLength`)) true)))