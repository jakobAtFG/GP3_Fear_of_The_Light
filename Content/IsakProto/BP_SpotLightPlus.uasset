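; BP_SpotLightPlus is an interactable spotlight that reveals hidden messages on actors it shines on.
; Overlap events track whether an actor is in the light cone, store it, and hide its message when it leaves.
; While lit and overlapped, Tick traces visibility from the light to that actor, revealing the message if unobstructed and hiding it otherwise.
; OnInteract sets or toggles the light, without itself hiding the message.
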(event `self.ReceiveActorBeginOverlap`
  (params (OtherActor :type "Actor Object Reference"))
  (set `self.InLightCone` true)
  (set `self.OtherActor` OtherActor))

(event `self.ReceiveActorEndOverlap`
  (params (OtherActor :type "Actor Object Reference"))
  (set `self.InLightCone` false)
  (message `/Game/IsakProto/Player/I_Revealable.OnHide` OtherActor))

(event `self.ReceiveTick`
  (params (DeltaSeconds :type "Float (single-precision)"))
  (bind _otheractor (`self.OtherActor`))
  (if (and (`self.InLightCone`) (`self.IsLightActive`))
    (bind (_outhit _returnvalue) (`KismetSystemLibrary.LineTraceSingle` (`SceneComponent.K2_GetComponentLocation` (`self.SpotLight`)) (`self.K2_GetActorLocation` (`self.OtherActor`)) "TraceTypeQuery1"))
    (if _returnvalue
      (message `/Game/IsakProto/Player/I_Revealable.OnHide` _otheractor)
      (else
        (message `/Game/IsakProto/Player/I_Revealable.OnReveal` _otheractor)))))

(event `/Game/BP/BI_Interactable.OnInteract`
  (params (bIsActive :type Boolean) (InteractionType :type "/Game/BP/E_InteractionType Enum" :default "NewEnumerator0"))
  (switch `/Game/BP/E_InteractionType` InteractionType
    (:`NewEnumerator0`
      (if bIsActive
        (set `self.IsLightActive` true :!label _label)
        (`SceneComponent.SetVisibility` (`self.SpotLight`) true false)
        (else
          (set `self.IsLightActive` false :!label _label_2)
          (`SceneComponent.SetVisibility` (`self.SpotLight`) false false))))
    (:`NewEnumerator2`
      (if (`self.IsLightActive`)
        (goto _label_2)
        (else
          (goto _label))))))

(fn `UserConstructionScript`)