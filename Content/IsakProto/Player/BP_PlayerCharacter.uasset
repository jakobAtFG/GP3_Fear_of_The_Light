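; Player character Blueprint with move and look input, camera-shake head bob, a light-exposure state and a toggleable heat vision.
; Input events drive actor-relative movement and controller rotation, while Tick starts a walk or idle camera shake every frame based on velocity.
; Reveal and hide events flip an in-light flag with debug prints.
; The E key toggles heat vision by showing or hiding a Plane component.
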(event `self.ReceiveTick`
  (params (DeltaSeconds :type "Float (single-precision)"))
  (`self.OnHeadBob`))

(event `/Game/IsakProto/Player/I_Controllable.OnLook`
  (params (Horizontal :type "Float (double-precision)") (Vertical :type "Float (double-precision)"))
  (`self.AddControllerPitchInput` Vertical)
  (`self.AddControllerYawInput` Horizontal))

(event `/Game/IsakProto/Player/I_Controllable.OnMove`
  (params (Horizontal :type "Float (double-precision)") (Vertical :type "Float (double-precision)"))
  (`self.AddMovementInput` (+ (* Horizontal (`self.GetActorRightVector`)) (* Vertical (`self.GetActorForwardVector`)))))

(event `OnHeadBob`
  (bind _returnvalue (`PlayerState.GetPlayerController` (`GameplayStatics.GetPlayerState` 0)))
  (if (> (`KismetMathLibrary.VSizeSquared` (`self.GetVelocity`)) 100.0)
    (`PlayerController.ClientStartCameraShake` :`self` _returnvalue :`Shake` "/Game/IsakProto/Player/CS_Walk.CS_Walk_C")
    (else
      (`PlayerController.ClientStartCameraShake` :`self` _returnvalue :`Shake` "/Game/IsakProto/Player/CS_Idle.CS_Idle_C"))))

(event `/Game/IsakProto/Player/I_Revealable.OnReveal`
  (if (not (`self.IsInLight`))
    (set `self.IsInLight` true)
    (`KismetSystemLibrary.PrintString` "IN LIGHT")))

(event `/Game/IsakProto/Player/I_Revealable.OnHide`
  (if (`self.IsInLight`)
    (set `self.IsInLight` false)
    (`KismetSystemLibrary.PrintString` "NOT IN LIGHT")))

(event `Key|E`
  (params (Key :type "Key Structure"))
  (:`Pressed`
    (set `self.HeatVisionEnabled` (not (`self.HeatVisionEnabled`)))
    (`SceneComponent.SetVisibility` (`self.Plane`) (`self.HeatVisionEnabled`) false)))

(fn `UserConstructionScript`)