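; BP_PatrolRoute is a spline actor that serves patrol waypoints one at a time.
; GetSplinePointAsLocation returns the world location of the spline point at the current index, and IncrementPatrolRoute steps that index by a direction modifier.
; Reaching the point count flips the direction to backward but also destroys the route actor, while an index at or below zero sets the direction forward.
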(event `IncrementPatrolRoute`
  (set `self.Index` (+ (`self.Index`) (`self.DirectionModifier`)))
  (if (>= (`self.Index`) (- (`SplineComponent.GetNumberOfSplinePoints` (`self.Spline`)) 0))
    (set `self.DirectionModifier` -1)
    (`self.K2_DestroyActor`)
    (elif (<= (`self.Index`) 0)
      (set `self.DirectionModifier` 1))))

(fn `Get Spline Point as Location`
  (returns (Location :type "Vector Structure"))
  (return (`SplineComponent.GetLocationAtSplinePoint` (`self.Spline`) (`self.Index`) "World")))

(fn `UserConstructionScript`)