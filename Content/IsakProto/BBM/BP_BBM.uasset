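; BP_BBM is an enemy that chases targets with AIMoveTo, supplies a patrol route and radar tag, and jump-scares the player to death.
; Overlapping its death range starts the scare and arms a per-tick kill cam that, given line of sight, turns the view to it, unpossesses the player and deals delayed damage.
; Flashes spawn an actor and animate emission on a dynamic material.
; GameManager save events store and restore its location by display name.
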(event `self.ReceiveBeginPlay`
  (bind _mesh (`self.Mesh`))
  (`|ExecutionSequence`
    (:`then_0`
      (bind _asgame_manager (cast `GameManager` (`GameplayStatics.GetGameInstance`)))
      (add `GameManager.OnSaveRequested` _asgame_manager (delegate `OnSaveRequested_Event`))
      (add `GameManager.OnSaveDataLoaded` _asgame_manager (delegate `OnSaveDataLoaded_Event`))
      (bind _returnvalue (`KismetMaterialLibrary.CreateDynamicMaterialInstance` "/Game/Art/3D/Characters/BigBoyMoth/NewBBM/MI_BigBoiMot.MI_BigBoiMot"))
      (bind _output_get (set `self.Material` _returnvalue))
      (`MaterialInstanceDynamic.SetScalarParameterValue` _output_get "Emission Strength" 0.0)
      (`PrimitiveComponent.SetMaterial` _mesh 0 _output_get)
      (`PrimitiveComponent.SetMaterial` _mesh 1 _output_get)
      (set `self.Player` (`GameplayStatics.GetPlayerCharacter` 0)))
    (:`then_1`
      (`self.SetupEyeBalls`))))

(event `OnSaveDataLoaded_Event`
  (params (SaveGame :type "GP3SaveGame Object Reference"))
  (bind (_value _returnvalue) (`BlueprintMapLibrary.Map_Find` (`GP3SaveGame.EnemyStartLocations` SaveGame) (`KismetSystemLibrary.GetDisplayName` self)))
  (if _returnvalue
    (`self.K2_SetActorLocation` _value)))

(event `OnSaveRequested_Event`
  (params (SaveGame :type "GP3SaveGame Object Reference"))
  (`BlueprintMapLibrary.Map_Add` (`GP3SaveGame.EnemyStartLocations` SaveGame) (`KismetSystemLibrary.GetDisplayName` self) (`self.K2_GetActorLocation`)))

(event `/Game/IsakProto/BBM/BPI_BBM.OnChase`
  (params (ChaseTarget :type "Actor Object Reference"))
  (`|AIMoveTo` self (0.0 0.0 0.0) ChaseTarget))

(event `/Game/IsakProto/BBM/BPI_BBM.OnFlash`
  (bind _returnvalue (`|SpawnActorFromClass` (`self.Flash`) (`self.GetTransform`) "Undefined" "MultiplyWithRoot" null null))
  (`self.SetOwner` _returnvalue self)
  ;[1 1 1] Finished does not trigger if play from start is triggered before finished
  (bind (_direction _emission_strength) (`Timeline|FlashEmissionTimeline` :!via `PlayFromStart`)
    (:`Update`
      (`MaterialInstanceDynamic.SetScalarParameterValue` (`self.Material`) "Emission Strength" _emission_strength))
    (:`Finished`
      ;;[1 1 1] Added backup destruction logic to flash
      (`self.K2_DestroyActor` _returnvalue))))

(event `/Game/IsakProto/BBM/BPI_BBM.OnSearch`)

(event `self.Death Range.OnComponentBeginOverlap`
  (params (OverlappedComponent :type "PrimitiveComponent Object Reference") (OtherActor :type "Actor Object Reference") (OtherComp :type "PrimitiveComponent Object Reference") (OtherBodyIndex :type Integer) (bFromSweep :type Boolean) (SweepResult :type "HitResult Structure (by ref)"))
  (if (== OtherActor (`GameplayStatics.GetPlayerCharacter` 0))
    (`AudioComponent.Play` (`self.SFX_ALIEN`) 0.0)
    (`|PlayMontage` (`self.Mesh`) "/Game/Art/3D/Characters/BigBoyMoth/NewBBM/AM_BBM_JumpScare.AM_BBM_JumpScare"
      (:`then`
        (set `self.KillPlayer` true)))))

(event `OnKillPlayer`
  (bind _returnvalue (`GameplayStatics.GetPlayerController` 0))
  (bind _player (`self.Player`))
  (bind _player_2 (`self.Player`))
  (if (`self.KillPlayer`)
    (bind (_outhit _returnvalue_2) (`KismetSystemLibrary.LineTraceSingle` (`self.K2_GetActorLocation`) (`self.K2_GetActorLocation` _player_2) "TraceTypeQuery1" false (`|MakeArray` _player_2 self :!type "Actor Object Reference")))
    (if (not _returnvalue_2)
      (`Controller.SetControlRotation` _returnvalue (`KismetMathLibrary.RInterpTo` (`Controller.GetControlRotation` _returnvalue) (`KismetMathLibrary.FindLookAtRotation` (`self.K2_GetActorLocation` _player) (`self.K2_GetActorLocation`)) (`GameplayStatics.GetWorldDeltaSeconds`) 10.0))
      (`self.SetActorHiddenInGame` _player true)
      (`Controller.UnPossess` _returnvalue)
      (`KismetSystemLibrary.Delay` 2.0)
      (bind _asgp3character (cast `GP3Character` (`self.Player`)))
      (`HealthComponent.TakeDamage` (`GP3Character.HealthComponent` _asgp3character) 100.0)
      (else
        (set `self.KillPlayer` false)))))

(event `self.ReceiveTick`
  (params (DeltaSeconds :type "Float (single-precision)"))
  (bind _sfx_bbm_footstepsquick (`self.SFX_BBM_FOOTSTEPSQUICK`))
  (`self.OnKillPlayer`)
  (if (and (> (`KismetMathLibrary.VSizeXY` (`self.GetVelocity`)) 50.0) (`AudioComponent.IsPlaying` (`self.SFX_BBM_FOOTSTEPSQUICK`)) (`self.bIsStanding`))
    (`AudioComponent.SetPaused` _sfx_bbm_footstepsquick false)
    (else
      (`AudioComponent.SetPaused` _sfx_bbm_footstepsquick true))))

(fn `GetGameplayTags`
  (returns (GameplayTagContainer :type "GameplayTagContainer Structure"))
  (return (struct :`GameplayTags` (struct :`(TagName` "RadarDetectable.Enemy")))))

(fn `OnPatrol`
  (returns (PatrolRoute :type "/Game/IsakProto/BBM/BP_PatrolRoute Object Reference"))
  (return (`self.PatrolRoute`)))

(fn `SetupEyeBalls`
  (`SceneComponent.K2_AttachToComponent` (`self.EyeSphere_R`) (`self.Mesh`) "face_008_R_012" "SnapToTarget" "KeepRelative" "KeepWorld" true)
  (`SceneComponent.K2_AttachToComponent` (`self.EyeSphere_L`) (`self.Mesh`) "face_008_L_012" "SnapToTarget" "KeepRelative" "KeepWorld" true))

(fn `UserConstructionScript`)