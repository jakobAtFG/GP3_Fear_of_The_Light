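; BP_BBM_Flash is a short-lived light flash tied to BP_BBM that reveals a message on the player while its light reaches them.
; Overlap flags the player inside the light sphere, and leaving hides the message.
; Each tick, a visibility trace from the point light, ignoring BP_BBM actors, hides the message on a hit and reveals it otherwise.
; A short lifespan set at BeginPlay serves as backup destruction.
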(event `self.ReceiveActorBeginOverlap`
  (params (OtherActor :type "Actor Object Reference"))
  (bind _returnvalue (`GameplayStatics.GetPlayerCharacter` 0))
  (if (== OtherActor _returnvalue)
    (set `self.IsInLightSphere` true)
    (set `self.OtherActor` _returnvalue)))

(event `self.ReceiveActorEndOverlap`
  (params (OtherActor :type "Actor Object Reference"))
  (set `self.IsInLightSphere` false)
  (message `/Game/IsakProto/Player/I_Revealable.OnHide` (`GameplayStatics.GetPlayerCharacter` 0)))

(event `self.ReceiveTick`
  (params (DeltaSeconds :type "Float (single-precision)"))
  (bind _otheractor (`self.OtherActor`))
  (if (`self.IsInLightSphere`)
    (bind _outactors (`GameplayStatics.GetAllActorsOfClass` "/Game/IsakProto/BBM/BP_BBM.BP_BBM_C"))
    (bind (_outhit _returnvalue) (`KismetSystemLibrary.LineTraceSingle` (`SceneComponent.K2_GetComponentLocation` (`self.PointLightComponent`)) (`self.K2_GetActorLocation` (`self.OtherActor`)) "TraceTypeQuery1" false _outactors))
    (if _returnvalue
      (message `/Game/IsakProto/Player/I_Revealable.OnHide` _otheractor)
      (else
        (message `/Game/IsakProto/Player/I_Revealable.OnReveal` _otheractor)))))

(event `self.ReceiveBeginPlay`
  ;[1 1 1] Backup destruction if BBM fails to due multiple flashes
  (`self.SetLifeSpan` 1.0))

(fn `UserConstructionScript`)