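; Interactive spotlight that reveals hidden messages on an actor inside its beam.
; BeginPlay scales the cone to match attenuation radius and inner angle; while overlapped, Tick line-traces visibility to the last entered actor, calling reveal when unobstructed, hide otherwise.
; OnInteract sets or toggles the light, with optional random-delay flickering.
; Externally triggered EMP events play shutdown and recovery timelines with Niagara effects, driving intensity and child-lamp emission together.
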(event `self.ReceiveBeginPlay`
  (bind _returnvalue (/ (`LocalLightComponent.AttenuationRadius` (`self.SpotLight`)) 110.0))
  (bind _returnvalue_2 (/ (`SpotLightComponent.InnerConeAngle` (`self.SpotLight`)) 24.0))
  (`SceneComponent.SetWorldScale3D` (`self.SpotLight`) (`KismetMathLibrary.MakeVector` _returnvalue _returnvalue _returnvalue))
  (`SceneComponent.SetRelativeScale3D` (`self.Cone`) (`KismetMathLibrary.MakeVector` _returnvalue_2 _returnvalue_2 1.0))
  (set `self.BaseLightIntensity` (`LightComponentBase.Intensity` (`self.SpotLight`)))
  (bind _asbp_lamp (cast `/Game/BP/BP_Lamp` (`ChildActorComponent.ChildActor` (`self.LampChildActor`))))
  (set `self.BP Lamp` _asbp_lamp)
  (if (`self.IsFlickering`)
    (`self.StartFlickering`)))

(event `self.ReceiveActorBeginOverlap`
  (params (OtherActor :type "Actor Object Reference"))
  (set `self.InLightCone` true)
  (set `self.OtherActor` OtherActor))

(event `self.ReceiveActorEndOverlap`
  (params (OtherActor :type "Actor Object Reference"))
  (set `self.InLightCone` false)
  (message `/Game/IsakProto/Player/I_Revealable.OnHide` OtherActor))

(event `self.ReceiveTick`
  (params (DeltaSeconds :type "Float (single-precision)"))
  (bind _otheractor (`self.OtherActor`))
  (if (and (`self.InLightCone`) (`self.IsLightActive`))
    (bind (_outhit _returnvalue) (`KismetSystemLibrary.LineTraceSingle` (`SceneComponent.K2_GetComponentLocation` (`self.SpotLight`)) (`self.K2_GetActorLocation` (`self.OtherActor`)) "TraceTypeQuery1"))
    (if _returnvalue
      (message `/Game/IsakProto/Player/I_Revealable.OnHide` _otheractor)
      (else
        (message `/Game/IsakProto/Player/I_Revealable.OnReveal` _otheractor)))))

(event `/Game/BP/BI_Interactable.OnInteract`
  (params (bIsActive :type Boolean) (InteractionType :type "/Game/BP/E_InteractionType Enum" :default "NewEnumerator0"))
  (switch `/Game/BP/E_InteractionType` InteractionType
    (:`NewEnumerator0`
      (if bIsActive
        (set `self.IsLightActive` true :!label _label)
        (`SceneComponent.SetVisibility` (`self.SpotLight`) true false)
        (if (`self.IsFlickering`)
          (`self.StartFlickering`)
          (else
            (`/Game/BP/BP_Lamp.SetEmissionStrength` (`self.BP Lamp`) 1.0)))
        (else
          (set `self.IsLightActive` false :!label _label_2)
          (`SceneComponent.SetVisibility` (`self.SpotLight`) false false)
          (message `/Game/IsakProto/Player/I_Revealable.OnHide` (`self.OtherActor`))
          (if (`self.IsFlickering`)
            (`self.StopFlickering`)
            (else
              (`/Game/BP/BP_Lamp.SetEmissionStrength` (`self.BP Lamp`) 0.0))))))
    (:`NewEnumerator2`
      (if (`self.IsLightActive`)
        (goto _label_2)
        (else
          (goto _label))))))

(event `StartFlickering`
  ;[1 1 1] Flickering
  (`KismetSystemLibrary.Delay` (`KismetMathLibrary.RandomFloatInRange` 0.0 1.0))
  (bind (_direction _emission_strength_multiplier) (`Timeline|FlickerTimeline` :!via `PlayFromStart` :!label _label_3)
    (:`Update`
      (`/Game/BP/BP_Lamp.SetEmissionStrength` (`self.BP Lamp`) _emission_strength_multiplier)
      (`self.SetLightIntensity` _emission_strength_multiplier))
    (:`Finished`
      (`self.StartFlickering`))))

(event `StopFlickering`
  ;[1 1 1] Flickering
  (`|ExecutionSequence`
    (:`then_0`
      (goto _label_3 :!via `Stop`))
    (:`then_1`
      (`/Game/BP/BP_Lamp.SetEmissionStrength` (`self.BP Lamp`) 1.0)
      (`self.SetLightIntensity` 1.0))))

(event `self.TurnOffLight`
  ;[1 1 1] EMP (Both events must be triggered from elsewhere)
  (if (not (`self.EMP Active`))
    (set `self.EMP Active` true)
    (if (`self.IsFlickering`)
      (`self.StopFlickering`))
    (`SceneComponent.SetVisibility` (`self.FXS_EMP_Distortion`) true false)
    (bind (_direction _emission_strength_multiplier) (`Timeline|EMPReceivedTimeline` :!via `PlayFromStart` :!label _label_4)
      (:`Update`
        (`/Game/BP/BP_Lamp.SetEmissionStrength` (`self.BP Lamp`) _emission_strength_multiplier)
        (`self.SetLightIntensity` _emission_strength_multiplier))
      (:`Finished`
        (`SceneComponent.SetVisibility` (`self.FXS_EMP_Distortion`) false false)
        (`NiagaraFunctionLibrary.SpawnSystemAttached` "/Game/VFX/NS_ElectricSpark1.NS_ElectricSpark1" (`self.SpotLight`) "None" (0.0 0.0 0.0) (struct) "KeepRelativeOffset")
        (set `self.IsLightActive` false)
        (message `/Game/IsakProto/Player/I_Revealable.OnHide` (`self.OtherActor`))))))

(event `self.TurnOnLight`
  ;[1 1 1] EMP (Both events must be triggered from elsewhere)
  (`|ExecutionSequence`
    (:`then_0`
      (goto _label_4 :!via `Stop`))
    (:`then_1`
      (bind (_direction _emission_strength_multiplier) (`Timeline|EMPDoneTimeline` :!via `PlayFromStart`)
        (:`Update`
          (`/Game/BP/BP_Lamp.SetEmissionStrength` (`self.BP Lamp`) _emission_strength_multiplier)
          (`self.SetLightIntensity` _emission_strength_multiplier))
        (:`Finished`
          (if (`self.IsFlickering`)
            (`self.StartFlickering`))
          (set `self.IsLightActive` true)
          (set `self.EMP Active` false))))))

(fn `SetLightIntensity`
  (params (`Intensity Multiplier` :type "Float (double-precision)"))
  (`LightComponent.SetIntensity` (`self.SpotLight`) (* (`self.BaseLightIntensity`) `Intensity Multiplier`)))

(fn `UserConstructionScript`)