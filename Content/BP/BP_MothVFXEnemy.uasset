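; Moth enemy with particle-effect visuals and audio that attacks its character target on contact.
; Overlapping the DeathRadius starts a delayed loop that calls AttackPlayer and plays a sound, with no check that the overlap persists.
; ChaseCharachterChange raises effect intensity and audio pitch and volume while chasing, restoring them otherwise.
; A temporary game-over function and AI move-to experiments remain in the graph but are never run.
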(event `self.ReceiveBeginPlay`)

(event `self.ReceiveTick`
  (params (DeltaSeconds :type "Float (single-precision)")))

(event `self.DeathRadius.OnComponentBeginOverlap`
  (params (OverlappedComponent :type "PrimitiveComponent Object Reference") (OtherActor :type "Actor Object Reference") (OtherComp :type "PrimitiveComponent Object Reference") (OtherBodyIndex :type Integer) (bFromSweep :type Boolean) (SweepResult :type "HitResult Structure (by ref)"))
  ;[1 1 1] Temporary Death
  (if (== OtherActor (`self.CharacterTarget`)) :!label _label
    (`KismetSystemLibrary.PrintText` "Attack")
    (`self.AttackPlayer`)
    (`AudioComponent.Play` (`self.SFX_FOOTSTEP_10`) 0.0)
    (`KismetSystemLibrary.Delay` (`self.AttackDelay`))
    (goto _label)))

(event `self.ChaseCharachterChange`
  ;[1 1 1] Change of looks when chasing
  (if (`self.bIsChasing`)
    (`NiagaraComponent.SetVariableFloat` (`self.FXS_MothPrototype`) "Intensity" 20.0)
    (`AudioComponent.SetPitchMultiplier` (`self.Audio`) 2.0)
    (`AudioComponent.SetVolumeMultiplier` (`self.Audio`) 2.0)
    (else
      (`NiagaraComponent.SetVariableFloat` (`self.FXS_MothPrototype`) "Intensity" 4.0)
      (`AudioComponent.SetPitchMultiplier` (`self.Audio`) 1.0)
      (`AudioComponent.SetVolumeMultiplier` (`self.Audio`) 1.0))))

(fn `TempDeathFunction`
  (bind _returnvalue (`|CreateWidget` "/Game/WBP/WBP_GameOver_PROT.WBP_GameOver_PROT_C"))
  (`UserWidget.AddToViewport` _returnvalue 0)
  (`GameplayStatics.SetGamePaused` true)
  (set `PlayerController.bShowMouseCursor` true (`GameplayStatics.GetPlayerController` 0)))

(fn `UserConstructionScript`)