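; Test player character with battery-powered radar and vision tools, plus lit/unlit tracking that counts strikes.
; Q and E toggle the vision plane and radar screen exclusively; Tick drains BatteryComponent, hides unpowered tools and updates the battery HUD.
; Tick also drives speed-based footstep pitch and head-bob camera shakes, and prints debug tool names.
; Scroll inputs forward to ToolManager, and Escape or U opens the main menu.
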(event `self.OnReveal`
  (if (not (`self.PlayerIsLitUp`))
    (set `self.PlayerIsLitUp` true)
    (bind _output_get (set `self.Strikes` (+ (`self.Strikes`) 1)))
    (`KismetSystemLibrary.PrintString` "lit")
    (`KismetSystemLibrary.PrintString` (`KismetStringLibrary.Conv_IntToString` _output_get))))

(event `self.OnHide`
  (if (`self.PlayerIsLitUp`)
    (set `self.PlayerIsLitUp` false)
    (`KismetSystemLibrary.PrintString` "not lit")))

(event `Key|Escape`
  (params (Key :type "Key Structure"))
  (:`Pressed`
    (`GameplayStatics.OpenLevel` "LV_AlphaMainMenu" :!label _label)))

(event `Key|U`
  (params (Key :type "Key Structure"))
  (:`Pressed`
    (goto _label)))

(event `self.ReceiveBeginPlay`
  (bind _batterycomponent (`self.BatteryComponent`))
  (`SceneComponent.SetVisibility` (`self.BP_RadarScreen`) false true)
  (`SceneComponent.SetVisibility` (`self.Plane`) false true)
  (bind _returnvalue (`|CreateWidget` "/Game/WBP/WBP_BatteryHUD.WBP_BatteryHUD_C" null (/ (`BatteryComponent.CurrentPower` _batterycomponent) (`BatteryComponent.MaxPower` _batterycomponent))))
  (bind _output_get (set `self.BatteryHUD` _returnvalue))
  (`UserWidget.AddToViewport` _output_get 0))

(event `Key|Q`
  (params (Key :type "Key Structure"))
  (:`Pressed`
    (`SceneComponent.ToggleVisibility` (`self.Plane`) true)
    (`SceneComponent.SetVisibility` (`self.BP_RadarScreen`) false true)))

(event `Key|E`
  (params (Key :type "Key Structure"))
  (:`Pressed`
    (`SceneComponent.ToggleVisibility` (`self.BP_RadarScreen`) true)
    (`SceneComponent.SetVisibility` (`self.Plane`) false true)))

(event `self.ReceiveTick`
  (params (DeltaSeconds :type "Float (single-precision)"))
  (bind _batterycomponent (`self.BatteryComponent`))
  (`|ExecutionSequence`
    (:`then_0`
      (`self.PlayFootsteps`)
      (`self.OnHeadBob`)
      (`|ExecutionSequence`
        (:`then_0`
          (if (`SceneComponent.bVisible` (`self.BP_RadarScreen`))
            (bind _returnvalue (`BatteryComponent.Consume` (`self.BatteryComponent`) "RADAR"))
            (if (not _returnvalue)
              (`SceneComponent.SetVisibility` (`self.BP_RadarScreen`) false true))))
        (:`then_1`
          (if (`SceneComponent.bVisible` (`self.Plane`))
            (bind _returnvalue_2 (`BatteryComponent.Consume` (`self.BatteryComponent`) "HEAT_VISION"))
            (if (not _returnvalue_2)
              (`SceneComponent.SetVisibility` (`self.Plane`) false true))))
        (:`then_2`
          (`/Game/WBP/WBP_BatteryHUD.SetPercent` (`self.BatteryHUD`) (/ (`BatteryComponent.CurrentPower` _batterycomponent) (`BatteryComponent.MaxPower` _batterycomponent))))))
    (:`then_1`
      (switch `int` (`KismetMathLibrary.FTrunc` (`self.FloatValue`))
        (:`0`
          (`KismetSystemLibrary.PrintString` "NONE"))
        (:`1`
          (`KismetSystemLibrary.PrintString` "EMP"))
        (:`2`
          (`KismetSystemLibrary.PrintString` "RADAR"))
        (:`3`
          (`KismetSystemLibrary.PrintString` "HEAT VISION"))))))

(event `PlayFootsteps`
  (bind _sfx_footsteps_loop_1 (`self.SFX_FOOTSTEPS_LOOP_1`))
  (bind _sfx_footsteps_loop_1_2 (`self.SFX_FOOTSTEPS_LOOP_1`))
  (bind _returnvalue (`KismetMathLibrary.VSizeXY` (`self.GetVelocity`)))
  (if (> _returnvalue 50.0)
    (`AudioComponent.SetPaused` _sfx_footsteps_loop_1 false)
    (if (> _returnvalue 150.0)
      (if (> _returnvalue 450.0)
        (`AudioComponent.SetPitchMultiplier` _sfx_footsteps_loop_1_2 1.2)
        (else
          (`AudioComponent.SetPitchMultiplier` _sfx_footsteps_loop_1_2 1.0)))
      (else
        (`AudioComponent.SetPitchMultiplier` _sfx_footsteps_loop_1_2 0.8)))
    (else
      (`AudioComponent.SetPaused` _sfx_footsteps_loop_1 true))))

(event `InputAction|ItemScrollerUp`
  (params (Key :type "Key Structure"))
  (:`Pressed`
    (`ToolManager.IncreaseWeaponIndex` (`self.ToolManager`) 0.0)))

(event `OnHeadBob`
  (bind _returnvalue (`KismetMathLibrary.VSizeXY` (`self.GetVelocity`)))
  (bind _returnvalue_2 (`PlayerState.GetPlayerController` (`GameplayStatics.GetPlayerState` 0)))
  (if (`self.Headbobbing`)
    (if (> _returnvalue 50.0)
      (if (> _returnvalue 150.0)
        (if (> _returnvalue 450.0)
          (`PlayerController.ClientStartCameraShake` :`self` _returnvalue_2 :`Shake` "/Game/IsakProto/Player/CS_Sprint.CS_Sprint_C")
          (else
            (`PlayerController.ClientStartCameraShake` :`self` _returnvalue_2 :`Shake` "/Game/IsakProto/Player/CS_Walk.CS_Walk_C")))
        (else
          (`PlayerController.ClientStartCameraShake` :`self` _returnvalue_2 :`Shake` "/Game/IsakProto/Player/CS_Crouched.CS_Crouched_C")))
      (else
        (`PlayerController.ClientStartCameraShake` :`self` _returnvalue_2 :`Shake` "/Game/IsakProto/Player/CS_Idle.CS_Idle_C")))))

(event `InputAction|ItemScrollerDown`
  (params (Key :type "Key Structure"))
  (:`Pressed`
    (`ToolManager.DecreaseWeaponIndex` (`self.ToolManager`) 0.0)))

(fn `UserConstructionScript`)