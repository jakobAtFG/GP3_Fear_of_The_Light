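; BP_Device_Radar is the handheld multi-tool device, switching its screen and sounds to match the player's current tool.
; On BeginPlay it binds to the player pawn's ToolManager tool-switch event.
; Radar and EMP each show their own screen and hide the other; None and Heat Vision leave screens unchanged.
; Radar starts tick and search audio, other tools stop it; a separate function toggles antenna visibility.
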(event `self.ReceiveBeginPlay`
  (add `ToolManager.OnToolSwitched` (`self.GetComponentByClass` (`GameplayStatics.GetPlayerPawn` 0) "/Script/GP3.ToolManager") (delegate `CustomEvent`)))

(event `CustomEvent`
  (params (CurrentTool :type "ETool Enum" :default "NONE"))
  (bind _sfx_radar_tick_normal (`self.SFX_RADAR_TICK_NORMAL`))
  (bind _sfx_radar_search (`self.SFX_RADAR_SEARCH`))
  (`self.SwitchToolVisual` CurrentTool)
  (switch `ETool` CurrentTool
    (:`NONE`
      (`AudioComponent.Stop` _sfx_radar_tick_normal :!label _label)
      (`AudioComponent.Stop` _sfx_radar_search))
    (:`RADAR`
      (`AudioComponent.Play` _sfx_radar_tick_normal 0.0)
      (`AudioComponent.Play` _sfx_radar_search 0.0))
    (:`HEAT_VISION`
      (goto _label))
    (:`EMP`
      (goto _label))))

(event `self.ReceiveTick`
  (params (DeltaSeconds :type "Float (single-precision)")))

(fn `SetAntennaVisibility`
  (params (`New Visibility` :type Boolean))
  (`SceneComponent.SetVisibility` (`self.MultiTool_Antenna`) `New Visibility` false))

(fn `SwitchToolVisual`
  (params (CurrentTool :type "ETool Enum" :default "NONE"))
  (switch `ETool` CurrentTool
    (:`RADAR`
      (`SceneComponent.SetVisibility` (`self.BP_RadarScreen`) true false)
      (`SceneComponent.SetVisibility` (`self.BP_EMPScreen`) false false))
    (:`EMP`
      (`SceneComponent.SetVisibility` (`self.BP_RadarScreen`) false false)
      (`SceneComponent.SetVisibility` (`self.BP_EMPScreen`) true false))))

(fn `UserConstructionScript`)