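; BP_Switch is a switch that relays interactions to other actors, built on a parent class that provides the base interact behavior.
; Its InteractEventFunction runs the parent logic, then calls InteractWithActors.
; That function loops over the Actors array and sends OnInteractMessage with IsActive and InteractionType to each valid actor implementing BI_Interactable, so targets are driven through the interface without casting.
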(event `self.ReceiveBeginPlay`
  (`parent.ReceiveBeginPlay`))

(fn `InteractEventFunction`
  (`parent.InteractEventFunction`)
  (`self.InteractWithActors`))

(fn `InteractWithActors`
  (bind _actors (`self.Actors`))
  (if (> (`KismetArrayLibrary.Array_Length` _actors) 0)
    (for _array_element _actors
      (`/Engine/EditorBlueprintResources/StandardMacros.IsValid` _array_element
        (:`Is Valid`
          (if (`KismetSystemLibrary.DoesImplementInterface` _array_element "/Game/BP/BI_Interactable.BI_Interactable_C")
            (message `/Game/BP/BI_Interactable.OnInteract` _array_element (`self.IsActive`) (`self.InteractionType`))))))))

(fn `UserConstructionScript`
  (`parent.UserConstructionScript`))