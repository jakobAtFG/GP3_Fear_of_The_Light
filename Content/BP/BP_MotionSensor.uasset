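; Motion sensor actor that switches a set of linked lights on and off as actors enter and leave its Cone trigger.
; The first detected actor plays a switch sound and turns the lights on; the last to leave starts a shutdown delay, rechecked before switching off.
; Lights are driven through BI_Interactable messages and start off one tick after BeginPlay.
; ToggleSensor only handles disabling, clearing detections and lights.
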(event `self.ReceiveBeginPlay`
  (`KismetSystemLibrary.DelayUntilNextTick`)
  (`self.ToggleLights` false))

(event `self.Cone.OnComponentBeginOverlap`
  (params (OverlappedComponent :type "PrimitiveComponent Object Reference") (OtherActor :type "Actor Object Reference") (OtherComp :type "PrimitiveComponent Object Reference") (OtherBodyIndex :type Integer) (bFromSweep :type Boolean) (SweepResult :type "HitResult Structure (by ref)"))
  (if (`self.SensorEnabled`)
    (if (not (`KismetArrayLibrary.Array_Contains` (`self.DetectedActors`) OtherActor))
      (if (not (> (`KismetArrayLibrary.Array_Length` (`self.DetectedActors`)) 0))
        (`self.ToggleLights` true)
        (`GameplayStatics.PlaySoundAtLocation` "/Game/Audio/Objects/SFX_SWITCH_Cue1.SFX_SWITCH_Cue1" (`self.K2_GetActorLocation`) (struct) 1.0 1.0 0.0 null null null null))
      (`KismetArrayLibrary.Array_AddUnique` (`self.DetectedActors`) OtherActor))))

(event `self.Cone.OnComponentEndOverlap`
  (params (OverlappedComponent :type "PrimitiveComponent Object Reference") (OtherActor :type "Actor Object Reference") (OtherComp :type "PrimitiveComponent Object Reference") (OtherBodyIndex :type Integer))
  (if (`self.SensorEnabled`)
    (if (`KismetArrayLibrary.Array_Contains` (`self.DetectedActors`) OtherActor)
      (`KismetArrayLibrary.Array_RemoveItem` (`self.DetectedActors`) OtherActor)
      (if (not (> (`KismetArrayLibrary.Array_Length` (`self.DetectedActors`)) 0))
        (`KismetSystemLibrary.Delay` (`self.ShutDownDelay`))
        (if (not (> (`KismetArrayLibrary.Array_Length` (`self.DetectedActors`)) 0))
          (`self.ToggleLights` false))))))

(fn `ToggleLights`
  (params (NewActive :type Boolean))
  (if (> (`KismetArrayLibrary.Array_Length` (`self.Lights`)) 0)
    (for _array_element (`self.Lights`)
      (`/Engine/EditorBlueprintResources/StandardMacros.IsValid` _array_element
        (:`Is Valid`
          (if (`KismetSystemLibrary.DoesImplementInterface` _array_element "/Game/BP/BI_Interactable.BI_Interactable_C")
            (message `/Game/BP/BI_Interactable.OnInteract` _array_element NewActive "NewEnumerator0")))))))

(fn `ToggleSensor`
  (params (NewActive :type Boolean))
  (if (not NewActive)
    (set `self.SensorEnabled` false)
    (`KismetArrayLibrary.Array_Clear` (`self.DetectedActors`))
    (`self.ToggleLights` false)))

(fn `UserConstructionScript`)