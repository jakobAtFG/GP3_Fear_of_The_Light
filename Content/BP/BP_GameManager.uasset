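; Game manager that handles win and lose end states and applies saved player settings on initialization.
; Win and lose events show their widget, pause the game and switch to UI input, with a shared flag preventing repeats.
; Init optionally wipes level and settings saves, then loads or creates SettingsSaveGame.
; Saved values drive a post-process material instance, sound class volumes and, a tick later, first-person character look and head-bob options.
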(event `self.OnWinGame`
  (bind _returnvalue (`GameplayStatics.GetPlayerController` 0))
  (if (not (`self.bIsGameEnded`))
    (bind _returnvalue_2 (`|CreateWidget` "/Game/WBP/WBP_GameWin_PROT.WBP_GameWin_PROT_C"))
    (bind _output_get (set `self.WinScreen` _returnvalue_2))
    (`UserWidget.AddToViewport` _output_get 0)
    (`GameplayStatics.SetGamePaused` true)
    (`WidgetBlueprintLibrary.SetInputMode_UIOnlyEx` _returnvalue (`self.WinScreen`))
    (set `PlayerController.bShowMouseCursor` true _returnvalue)
    (set `self.bIsGameEnded` true)))

(event `self.OnLoseGame`
  (bind _returnvalue (`GameplayStatics.GetPlayerController` 0))
  (if (not (`self.bIsGameEnded`))
    (bind _returnvalue_2 (`|CreateWidget` "/Game/WBP/WBP_GameOver.WBP_GameOver_C"))
    (bind _output_get (set `self.LoseSceen` _returnvalue_2))
    (`UserWidget.AddToViewport` _output_get 0)
    (`GameplayStatics.SetGamePaused` true)
    (`WidgetBlueprintLibrary.SetInputMode_UIOnlyEx` _returnvalue (`self.LoseSceen`))
    (set `PlayerController.bShowMouseCursor` true _returnvalue)
    (set `self.bIsGameEnded` true)))

(event `self.ReceiveInit`
  (bind _returnvalue (`GameplayStatics.GetPlayerCharacter` 0))
  (bind _settingssavegame (`self.SettingsSaveGame`))
  (bind (_x _y) (`KismetMathLibrary.BreakVector2D` (`/Game/WBP/SoundUI/SettingsSaveGame.MouseSensitivity` (`self.SettingsSaveGame`))))
  (`|ExecutionSequence`
    (:`then_0`
      (if (`self.DeleteSaveOnStart`)
        (bind _returnvalue_2 (`GameplayStatics.GetCurrentLevelName` true))
        (`GameplayStatics.DeleteGameInSlot` _returnvalue_2)))
    (:`then_1`
      (if (`self.DeleteSettingsOnStart`)
        (`GameplayStatics.DeleteGameInSlot` "SettingsSaveGame")))
    (:`then_2`
      (bind _returnvalue_3 (`GameplayStatics.DoesSaveGameExist` "SettingsSaveGame"))
      (if _returnvalue_3
        (bind _returnvalue_4 (`GameplayStatics.LoadGameFromSlot` "SettingsSaveGame"))
        (bind _assettings_save_game (cast `/Game/WBP/SoundUI/SettingsSaveGame` _returnvalue_4))
        (set `self.SettingsSaveGame` _assettings_save_game)
        (else
          (bind _returnvalue_5 (`GameplayStatics.CreateSaveGameObject` "/Game/WBP/SoundUI/SettingsSaveGame.SettingsSaveGame_C"))
          (`AsyncActionHandleSaveGame.AsyncSaveGameToSlot` _returnvalue_5 "SettingsSaveGame"
            (:`then`
              (set `self.SettingsSaveGame` _returnvalue_5))))))
    (:`then_3`
      (bind _returnvalue_6 (`KismetMaterialLibrary.CreateDynamicMaterialInstance` "/Game/Material/PPMI_Main.PPMI_Main"))
      (bind _output_get (set `self.PostProcessingMaterial` _returnvalue_6))
      (`MaterialInstanceDynamic.SetScalarParameterValue` _output_get "Brightness" (`/Game/WBP/SoundUI/SettingsSaveGame.Brightness` _settingssavegame))
      (`MaterialInstanceDynamic.SetScalarParameterValue` _output_get "Contrast" (`/Game/WBP/SoundUI/SettingsSaveGame.Contrast` _settingssavegame)))
    (:`then_4`
      (`GameplayStatics.SetBaseSoundMix` "/Game/Audio/Classes/SoundManagerMix.SoundManagerMix")
      (`|ExecutionSequence`
        (:`then_1`
          (`KismetSystemLibrary.DelayUntilNextTick`)
          (`|ExecutionSequence`
            (:`then_0`
              (for (_array_element _array_index) (`/Game/WBP/SoundUI/SettingsSaveGame.SoundVolumes` (`self.SettingsSaveGame`))
                (switch `int` _array_index
                  (:`0`
                    (`GameplayStatics.SetSoundMixClassOverride` "/Game/Audio/Classes/SoundManagerMix.SoundManagerMix" "/Game/Audio/Classes/SFX_MasterVolume.SFX_MasterVolume" _array_element 1.0 0.0))
                  (:`1`
                    (`GameplayStatics.SetSoundMixClassOverride` "/Game/Audio/Classes/SoundManagerMix.SoundManagerMix" "/Game/Audio/Classes/SFX_AmbienceSoundClass.SFX_AmbienceSoundClass" _array_element 1.0 0.0))
                  (:`2`
                    (`GameplayStatics.SetSoundMixClassOverride` "/Game/Audio/Classes/SoundManagerMix.SoundManagerMix" "/Game/Audio/Classes/SFX_SFXSoundClass.SFX_SFXSoundClass" _array_element 1.0 0.0)))))
            (:`then_1`
              (bind _asbp_first_person_character (cast `/Game/FirstPerson/Blueprints/BP_FirstPersonCharacter` (`GameplayStatics.GetPlayerCharacter` 0)))
              (set `/Game/FirstPerson/Blueprints/BP_FirstPersonCharacter.HeadBobbingOn` (`/Game/WBP/SoundUI/SettingsSaveGame.HeadBobSaveGame` (`self.SettingsSaveGame`)) _asbp_first_person_character))
            (:`then_2`
              (`|ExecutionSequence`
                (:`then_0`
                  (bind _asbp_first_person_character_2 (cast `/Game/FirstPerson/Blueprints/BP_FirstPersonCharacter` _returnvalue))
                  (set `GP3Character.HorizontalSensitivity` _x _asbp_first_person_character_2))
                (:`then_1`
                  (bind _asbp_first_person_character_3 (cast `/Game/FirstPerson/Blueprints/BP_FirstPersonCharacter` _returnvalue))
                  (set `GP3Character.VerticalSensitivity` _y _asbp_first_person_character_3))))
            (:`then_3`
              (for (_array_element_2 _array_index_2) (`/Game/WBP/SoundUI/SettingsSaveGame.InvertMouse` (`self.SettingsSaveGame`))
                (bind _asbp_first_person_character_4 (cast `/Game/FirstPerson/Blueprints/BP_FirstPersonCharacter` (`GameplayStatics.GetPlayerCharacter` 0)))
                (switch `int` _array_index_2
                  (:`0`
                    (if _array_element_2
                      (set `GP3Character.InvertHorizontal` -1.0 _asbp_first_person_character_4)
                      (else
                        (set `GP3Character.InvertHorizontal` 1.0 _asbp_first_person_character_4))))
                  (:`1`
                    (if _array_element_2
                      (set `GP3Character.InvertVertical` -1.0 _asbp_first_person_character_4)
                      (else
                        (set `GP3Character.InvertVertical` 1.0 _asbp_first_person_character_4)))))))))))))