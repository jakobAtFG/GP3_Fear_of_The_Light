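; A keycard pickup that grants the player a clearance level, shown as an "LV." text label set at construction.
; Interacting adds the level to the first-person character, closes the info widget, plays a sound, then hides the card and disables its trace detection collision rather than destroying it.
; On GameManager's save-loaded event, it hides or restores itself by comparing saved clearance to its own.
; It reports a Keycard radar-detectable gameplay tag.
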(event `self.ReceiveBeginPlay`
  (`parent.ReceiveBeginPlay`)
  (bind _asgame_manager (cast `GameManager` (`GameplayStatics.GetGameInstance`)))
  (add `GameManager.OnSaveDataLoaded` _asgame_manager (delegate `OnSaveDataLoaded_Event`)))

(event `OnSaveDataLoaded_Event`
  (params (SaveGame :type "GP3SaveGame Object Reference"))
  (bind _returnvalue (>= (`GP3SaveGame.ClearanceLevel` SaveGame) (`self.Clearance Level`)))
  (`self.SetActorHiddenInGame` _returnvalue)
  (`PrimitiveComponent.SetCollisionEnabled` (`self.LineTraceDetectionRange`) (select `bool` _returnvalue :`false` "QueryOnly" :`true` "NoCollision" :!type "ECollisionEnabled Enum")))

(fn `GetGameplayTags`
  (returns (GameplayTagContainer :type "GameplayTagContainer Structure"))
  (return (struct :`GameplayTags` (struct :`(TagName` "RadarDetectable.Keycard")))))

(fn `InteractEventFunction`
  (`parent.InteractEventFunction`)
  (bind _asbp_first_person_character (cast `/Game/FirstPerson/Blueprints/BP_FirstPersonCharacter` (`GameplayStatics.GetPlayerCharacter` 0)))
  (`/Game/FirstPerson/Blueprints/BP_FirstPersonCharacter.AddClearanceLevel` _asbp_first_person_character (`self.Clearance Level`))
  (`self.Close Info Widget`)
  (`self.SetActorHiddenInGame` true)
  (`PrimitiveComponent.SetCollisionEnabled` (`self.LineTraceDetectionRange`) "NoCollision")
  (`GameplayStatics.PlaySound2D` "/Game/Audio/SFX_PICKUP_ITEM.SFX_PICKUP_ITEM" 1.0 1.0 0.0 null null))

(fn `UserConstructionScript`
  (`parent.UserConstructionScript`)
  (`TextRenderComponent.K2_SetText` (`self.TextRender`) (`KismetTextLibrary.Conv_StringToText` (`KismetStringLibrary.Concat_StrStr` "LV. " (`KismetStringLibrary.Conv_IntToString` (`self.Clearance Level`))))))