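; BP_TimedSwitch is a timer actor that alternates between active and paused, sending its state to a list of linked actors.
; BeginPlay broadcasts the initial state, holding Tick off through an optional start delay.
; Tick runs at a construction-set interval, counting active or paused cycles and flipping IsActive at each limit.
; Each broadcast calls OnInteractMessage on valid actors implementing BI_Interactable.
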(event `self.ReceiveBeginPlay`
  ;[1 1 1] Start delay before tick starts.
  (`KismetSystemLibrary.DelayUntilNextTick`)
  (`self.SetActorTickEnabled` false)
  (`self.InteractWithActors`)
  (if (> (`self.StartDelay`) 0.0)
    (`KismetSystemLibrary.Delay` (`self.StartDelay`)))
  (`self.SetActorTickEnabled` true))

(event `self.ReceiveTick`
  (params (DeltaSeconds :type "Float (single-precision)"))
  (if (`self.IsActive`)
    ;[1 1 1] Active
    (bind _result (`/Engine/EditorBlueprintResources/StandardMacros.IncrementInt` (`self.CurrActiveIndex`))
      (:`  `
        (if (>= _result (`self.ActiveCycles`))
          (set `self.CurrActiveIndex` 0)
          ;[1 1 1] Reverse
          (set `self.IsActive` (not (`self.IsActive`)) :!label _label)
          (if (> (`KismetArrayLibrary.Array_Length` (`self.Actors`)) 0)
            (`self.InteractWithActors`)))))
    (else
      ;[1 1 1] Paused
      (bind _result_2 (`/Engine/EditorBlueprintResources/StandardMacros.IncrementInt` (`self.CurrPausedIndex`))
        (:`  `
          (if (>= _result_2 (`self.PauseCycles`))
            (set `self.CurrPausedIndex` 0)
            (goto _label)))))))

(fn `InteractWithActors`
  (for _array_element (`self.Actors`)
    (`/Engine/EditorBlueprintResources/StandardMacros.IsValid` _array_element
      (:`Is Valid`
        (if (`KismetSystemLibrary.DoesImplementInterface` _array_element "/Game/BP/BI_Interactable.BI_Interactable_C")
          (message `/Game/BP/BI_Interactable.OnInteract` _array_element (`self.IsActive`) "NewEnumerator0"))))))

(fn `UserConstructionScript`
  (`self.SetActorTickInterval` (`self.TickTimer`)))