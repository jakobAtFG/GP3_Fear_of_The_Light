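; BP_EmpGun is an EMP gun Blueprint that handles firing feedback for the first-person player character.
; PlayEmpSound calls EMPFire on the character's battery HUD, then after a short delay plays a disruptor sound ahead of the gun along its forward vector.
; EmpMisfire is unfinished: it only casts the player and logs failure, while an electric-spark Niagara effect meant for the radar device is left disconnected.
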(event `self.PlayEmpSound`
  (bind _asbp_first_person_character (cast `/Game/FirstPerson/Blueprints/BP_FirstPersonCharacter` (`GameplayStatics.GetPlayerCharacter` 0)))
  (`/Game/WBP/WBP_BatteryHUD.EMPFire` (`/Game/FirstPerson/Blueprints/BP_FirstPersonCharacter.BatteryHUD` _asbp_first_person_character))
  (`KismetSystemLibrary.Delay` 0.5)
  (`GameplayStatics.PlaySoundAtLocation` "/Game/Audio/Tools/SFX_DISRUPTOR_2.SFX_DISRUPTOR_2" (+ (* (`self.GetActorForwardVector`) 1000) (`self.K2_GetActorLocation`)) (struct) 1.0 1.0 0.0 null null null null))

(event `self.EmpMisfire`
  (bind _asbp_first_person_character (cast `/Game/FirstPerson/Blueprints/BP_FirstPersonCharacter` (`GameplayStatics.GetPlayerCharacter` 0))
    (:`CastFailed`
      (`KismetSystemLibrary.PrintString` "Cast Failed"))))

(fn `UserConstructionScript`)