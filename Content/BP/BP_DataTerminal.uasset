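; Interactable data terminal with an in-world widget screen listing doors and lights linked to it.
; BeginPlay builds a slot widget per Items entry, sorts it into the door or light box, and messages each linked actor its initial state.
; The InteractEventFunction override toggles terminal use, blending the view to or from the terminal while switching mouse cursor and move input.
; Older sphere-overlap cursor logic remains but is never bound.
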(event `self.ReceiveBeginPlay`
  (`parent.ReceiveBeginPlay`)
  (bind _aswbp_data_terminal_prot (cast `/Game/WBP/DataTerminal_PROT/WBP_DataTerminal_PROT` (`WidgetComponent.GetWidget` (`self.Widget`))))
  (set `self.As WBP Data Terminal PROT` _aswbp_data_terminal_prot)
  (set `self.Active` false)
  (for _array_element (`self.Items`)
    (bind _returnvalue (`|CreateWidget` "/Game/WBP/DataTerminal_PROT/WBP_DataTerminalSlot_PROT.WBP_DataTerminalSlot_PROT_C"))
    (bind (_itemname _isdoor _isactive _actor) (break `/Game/BP/F_DataTerminalItemProt` _array_element))
    (`/Game/WBP/DataTerminal_PROT/WBP_DataTerminalSlot_PROT.Initialize` _returnvalue _itemname _isdoor _isactive _actor)
    (if _isdoor
      (`PanelWidget.AddChild` (`/Game/WBP/DataTerminal_PROT/WBP_DataTerminal_PROT.DoorBox` (`self.As WBP Data Terminal PROT`)) _returnvalue)
      (else
        (`PanelWidget.AddChild` (`/Game/WBP/DataTerminal_PROT/WBP_DataTerminal_PROT.LightBox` (`self.As WBP Data Terminal PROT`)) _returnvalue)))
    (message `/Game/BP/BI_Interactable.OnInteract` _actor _isactive "NewEnumerator0")))

(event `self.ReceiveTick`
  (params (DeltaSeconds :type "Float (single-precision)"))
  (`parent.ReceiveTick` DeltaSeconds))

(event `TurnOnCursor`
  (params (OverlappedComponent :type "PrimitiveComponent Object Reference") (OtherActor :type "Actor Object Reference") (OtherComp :type "PrimitiveComponent Object Reference") (OtherBodyIndex :type Integer) (bFromSweep :type Boolean) (SweepResult :type "HitResult Structure (by ref)"))
  (bind _returnvalue (`GameplayStatics.GetPlayerController` 0))
  ;[1 1 1] Deprecated
  (if (== OtherActor (`GameplayStatics.GetPlayerCharacter` 0))
    (set `PlayerController.bShowMouseCursor` true _returnvalue)
    (`self.DisableInput` (`GameplayStatics.GetPlayerCharacter` 0) _returnvalue)))

(event `TurnOffCursor`
  (params (OverlappedComponent :type "PrimitiveComponent Object Reference") (OtherActor :type "Actor Object Reference") (OtherComp :type "PrimitiveComponent Object Reference") (OtherBodyIndex :type Integer))
  (bind _returnvalue (`GameplayStatics.GetPlayerController` 0))
  ;[1 1 1] Deprecated
  (if (== (stale `TurnOnCursor` OtherActor) (`GameplayStatics.GetPlayerCharacter` 0))
    (set `PlayerController.bShowMouseCursor` false _returnvalue)
    (`self.EnableInput` (`GameplayStatics.GetPlayerCharacter` 0) _returnvalue)))

(fn `InteractEventFunction`
  (bind _returnvalue (`GameplayStatics.GetPlayerController` 0))
  (`parent.InteractEventFunction`)
  (if (`self.Active`)
    (set `PlayerController.bShowMouseCursor` false _returnvalue)
    (`PlayerController.SetViewTargetWithBlend` _returnvalue (`GameplayStatics.GetPlayerCharacter` 0) 0.5 "VTBlend_Linear" 0.0 false)
    (`Controller.SetIgnoreMoveInput` _returnvalue false)
    (set `self.Active` false)
    (else
      (set `PlayerController.bShowMouseCursor` true _returnvalue)
      (`PlayerController.SetViewTargetWithBlend` _returnvalue self 0.5 "VTBlend_Linear" 0.0 false)
      (`Controller.SetIgnoreMoveInput` _returnvalue true)
      (set `self.Active` true))))

(fn `UserConstructionScript`
  (`parent.UserConstructionScript`))