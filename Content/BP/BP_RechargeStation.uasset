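; Interactable recharge station for the player's battery, tagged as a charging station for radar detection.
; Interacting finds the first-person character and toggles recharge on its BatteryComponent, while closing the on-screen info switches recharge off.
; Overlap events cache or clear that component reference.
; Tick polls the component's recharging state to show the sphere and unpause the recharge sound.
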(event `self.ReceiveBeginPlay`
  (`parent.ReceiveBeginPlay`)
  (`AudioComponent.SetPaused` (`self.SFX_RECHARGE_BATTERY`) true))

(event `self.ReceiveActorBeginOverlap`
  (params (OtherActor :type "Actor Object Reference"))
  (`parent.ReceiveActorBeginOverlap` OtherActor)
  (bind _output_get (set `self.Other Actor` OtherActor))
  (bind _asgp3character (cast `GP3Character` _output_get))
  (bind _returnvalue (`self.GetComponentByClass` _asgp3character "/Script/GP3.BatteryComponent"))
  (`/Engine/EditorBlueprintResources/StandardMacros.IsValid` _returnvalue
    (:`Is Valid`
      (set `self.PlayerBatteryComponent` _returnvalue))))

(event `self.ReceiveActorEndOverlap`
  (params (OtherActor :type "Actor Object Reference"))
  (`parent.ReceiveActorBeginOverlap` OtherActor)
  (bind _output_get (set `self.Other Actor` OtherActor))
  (cast `GP3Character` _output_get)
  (set `self.PlayerBatteryComponent` null))

(event `self.ReceiveTick`
  (params (DeltaSeconds :type "Float (single-precision)"))
  (bind _bisrecharging (`BatteryComponent.bIsRecharging` (`self.PlayerBatteryComponent`)))
  (`parent.ReceiveTick` DeltaSeconds)
  (`/Engine/EditorBlueprintResources/StandardMacros.IsValid` (`self.PlayerBatteryComponent`)
    (:`Is Valid`
      (`SceneComponent.SetVisibility` (`self.Sphere`) _bisrecharging false)
      (`AudioComponent.SetPaused` (`self.SFX_RECHARGE_BATTERY`) (not _bisrecharging)))))

(event `self.CloseInfoOnScreen`
  (`parent.CloseInfoOnScreen`)
  (bind _output_get (set `BatteryComponent.bIsRecharging` false (`self.PlayerBatteryComponent`)))
  (`SceneComponent.SetVisibility` (`self.Sphere`) _output_get false))

(fn `GetGameplayTags`
  (returns (GameplayTagContainer :type "GameplayTagContainer Structure"))
  (return (struct :`GameplayTags` (struct :`(TagName` "RadarDetectable.ChargingStation")))))

(fn `InteractEventFunction`
  (`parent.InteractEventFunction`)
  (bind _returnvalue (`GameplayStatics.GetActorOfClass` "/Game/FirstPerson/Blueprints/BP_FirstPersonCharacter.BP_FirstPersonCharacter_C"))
  (bind _output_get (set `self.PlayerCharacter` _returnvalue))
  (bind _output_get_2 (set `self.PlayerBatteryComponent` (`self.GetComponentByClass` _output_get "/Script/GP3.BatteryComponent")))
  (`/Engine/EditorBlueprintResources/StandardMacros.IsValid` _output_get_2
    (:`Is Valid`
      (`BatteryComponent.ToggleRecharge` _output_get_2))))

(fn `UserConstructionScript`
  (`parent.UserConstructionScript`))