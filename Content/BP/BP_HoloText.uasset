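; BP_HoloText is a text display actor, named as a hologram, that can be hidden or shown through interaction.
; The construction script applies StartText and StartColor to its TextRender component through SetTextAndColor.
; OnInteract sets the visibility of the scene root and its children to the inverse of IsActive, so an active state hides the text.
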(event `/Game/BP/BI_Interactable.OnInteract`
  (params (bIsActive :type Boolean) (InteractionType :type "/Game/BP/E_InteractionType Enum" :default "NewEnumerator0"))
  (`SceneComponent.SetVisibility` (`self.DefaultSceneRoot`) (not bIsActive) true))

(fn `SetTextAndColor`
  (params (Text :type Text) (Color :type "Color Structure"))
  (bind _textrender (`self.TextRender`))
  (`TextRenderComponent.K2_SetText` _textrender Text)
  (`TextRenderComponent.SetTextRenderColor` _textrender Color))

(fn `UserConstructionScript`
  (`self.SetTextAndColor` (`self.StartText`) (`self.StartColor`)))