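; Trigger volume that remotely fires an interaction on a list of actors when the player character walks into its box.
; On overlap by player 0's character, it loops through TriggeredActors and sends OnInteractMessage, flagged inactive, to each valid actor implementing BI_Interactable.
; An OnlyTriggerOnce option uses a Triggered flag to limit this to the first overlap; otherwise it fires on every entry.
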(event `self.Box.OnComponentBeginOverlap`
  (params (OverlappedComponent :type "PrimitiveComponent Object Reference") (OtherActor :type "Actor Object Reference") (OtherComp :type "PrimitiveComponent Object Reference") (OtherBodyIndex :type Integer) (bFromSweep :type Boolean) (SweepResult :type "HitResult Structure (by ref)"))
  (if (== OtherActor (`GameplayStatics.GetPlayerCharacter` 0))
    (if (`self.OnlyTriggerOnce`)
      (if (not (`self.Triggered`))
        (set `self.Triggered` true)
        (if (> (`KismetArrayLibrary.Array_Length` (`self.TriggeredActors`)) 0) :!label _label
          (for _array_element (`self.TriggeredActors`)
            (`/Engine/EditorBlueprintResources/StandardMacros.IsValid` _array_element
              (:`Is Valid`
                (if (`KismetSystemLibrary.DoesImplementInterface` _array_element "/Game/BP/BI_Interactable.BI_Interactable_C")
                  (message `/Game/BP/BI_Interactable.OnInteract` _array_element false "NewEnumerator0")
                  (if (`self.OnlyTriggerOnce`)
                    _)))))))
      (else
        (goto _label)))))

(fn `UserConstructionScript`)