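; BP_InteractableActor is a base interactable actor that shows an input prompt and responds to interaction.
; On BeginPlay it binds to OnInteract, which calls InteractEventFunction, an empty hook, and optionally disables further interaction after one use.
; Show and close events create and remove a WBP_InteractPrompt widget configured with key, text and position.
; Disabling works by making LineTraceDetectionRange ignore a custom trace channel.
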(event `self.ReceiveBeginPlay`
  (add `self.OnInteract` (delegate `OnInteract_Event`)))

(event `OnInteract_Event`
  (`KismetSystemLibrary.PrintString` "Logic Binded From BluePrint" false)
  (`self.InteractEventFunction`)
  (if (`self.bInteractOnlyOnce`)
    (`self.DisableInteraction`)))

(event `self.CloseInfoOnScreen`
  (`self.Close Info Widget`))

(event `self.ShowInfoOnScreen`
  (`self.Show Info Widget`))

(fn `Close Info Widget`
  (bind _interactionwidget (`self.InteractionWidget`))
  (`KismetSystemLibrary.PrintString` "close info on screen" false)
  (`/Engine/EditorBlueprintResources/StandardMacros.IsValid` _interactionwidget
    (:`Is Valid`
      (`Widget.RemoveFromParent` _interactionwidget))))

(fn `DisableInteraction`
  (`PrimitiveComponent.SetCollisionResponseToChannel` (`self.LineTraceDetectionRange`) "ECC_GameTraceChannel3" "ECR_Ignore"))

(fn `InteractEventFunction`)

(fn `Show Info Widget`
  (`KismetSystemLibrary.PrintString` "show info on screen" false)
  (bind _returnvalue (`|CreateWidget` "/Game/WBP/WBP_InteractPrompt.WBP_InteractPrompt_C" null (`self.Input Keycode`) (`self.Prompt Text`) (`self.PositionIndex`)))
  (bind _output_get (set `self.InteractionWidget` _returnvalue))
  (`UserWidget.AddToViewport` _output_get 0))

(fn `UserConstructionScript`)