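; Interactable pickup that grants the player the radar tool.
; On interact, it adds RADAR to the player pawn's ToolManager component, closes the info widget, and notifies the first-person character's BatteryHUD before running the parent interact logic.
; It returns the RadarDetectable.PickUp gameplay tag, identifying it as a radar-detectable pickup.
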(event `self.InteractEventFunction`
  (`ToolManager.AddTool` (`self.GetComponentByClass` (`GameplayStatics.GetPlayerPawn` 0) "/Script/GP3.ToolManager") "RADAR")
  (`self.Close Info Widget`)
  (bind _asbp_first_person_character (cast `/Game/FirstPerson/Blueprints/BP_FirstPersonCharacter` (`GameplayStatics.GetPlayerCharacter` 0)))
  (`/Game/WBP/WBP_BatteryHUD.AddTool` (`/Game/FirstPerson/Blueprints/BP_FirstPersonCharacter.BatteryHUD` _asbp_first_person_character))
  (`parent.InteractEventFunction`))

(fn `GetGameplayTags`
  (returns (GameplayTagContainer :type "GameplayTagContainer Structure"))
  (return (struct :`GameplayTags` (struct :`(TagName` "RadarDetectable.PickUp")))))

(fn `UserConstructionScript`
  (`parent.UserConstructionScript`))