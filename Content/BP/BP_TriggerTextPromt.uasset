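; Trigger volume that shows a configurable interact prompt widget while the first-person character overlaps its box.
; Begin overlap creates WBP_InteractPrompt with exposed key, text and position on first use, then reuses the cached instance.
; End overlap removes the prompt from the viewport.
; Optional OnlyTriggerOnce sets Triggered before the character cast, so any overlapping actor consumes the single use.
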(event `self.Box.OnComponentBeginOverlap`
  (params (OverlappedComponent :type "PrimitiveComponent Object Reference") (OtherActor :type "Actor Object Reference") (OtherComp :type "PrimitiveComponent Object Reference") (OtherBodyIndex :type Integer) (bFromSweep :type Boolean) (SweepResult :type "HitResult Structure (by ref)"))
  (bind _widget (`self.Widget`))
  (if (`self.OnlyTriggerOnce`)
    (if (not (`self.Triggered`))
      (set `self.Triggered` true)
      (cast `/Game/FirstPerson/Blueprints/BP_FirstPersonCharacter` OtherActor :!label _label)
      (`/Engine/EditorBlueprintResources/StandardMacros.IsValid` _widget
        (:`Is Valid`
          (`UserWidget.AddToViewport` _widget 0))
        (:`Is Not Valid`
          (bind _returnvalue (`|CreateWidget` "/Game/WBP/WBP_InteractPrompt.WBP_InteractPrompt_C" (`GameplayStatics.GetPlayerController` 0) (`self.Input Keycode`) (`self.Prompt Text`) (`self.Widget Position`)))
          (bind _output_get (set `self.Widget` _returnvalue))
          (`UserWidget.AddToViewport` _output_get 0))))
    (else
      (goto _label))))

(event `self.Box.OnComponentEndOverlap`
  (params (OverlappedComponent :type "PrimitiveComponent Object Reference") (OtherActor :type "Actor Object Reference") (OtherComp :type "PrimitiveComponent Object Reference") (OtherBodyIndex :type Integer))
  (`/Engine/EditorBlueprintResources/StandardMacros.IsValid` (`self.Widget`)
    (:`Is Valid`
      (cast `/Game/FirstPerson/Blueprints/BP_FirstPersonCharacter` OtherActor)
      (`Widget.RemoveFromParent` (`self.Widget`)))))

(fn `UserConstructionScript`)