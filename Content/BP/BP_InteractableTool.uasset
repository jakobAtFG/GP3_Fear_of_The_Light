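; Base pickup actor for the radar, heat vision and EMP tools, setting its tool type at BeginPlay by casting itself to child classes.
; On interact it plays a pickup sound, shows an equip-key prompt and hides itself.
; It stays alive until ToolManager signals a switch to that tool, then removes the prompt and destroys itself.
; It also destroys itself when GameManager's loaded save lists the tool as unlocked.
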(event `OnSwitchedToRadar_Event`
  (`/Engine/EditorBlueprintResources/StandardMacros.IsValid` (stale `self.InteractEventFunction` _returnvalue_2)
    (:`Is Valid`
      (`Widget.RemoveFromParent` (stale `self.InteractEventFunction` _returnvalue_2))
      (`self.K2_DestroyActor` :!label _label))))

(event `self.InteractEventFunction`
  (bind _returnvalue (`self.GetComponentByClass` (`GameplayStatics.GetPlayerPawn` 0) "/Script/GP3.ToolManager"))
  (`GameplayStatics.PlaySound2D` "/Game/Audio/SFX_PICKUP_ITEM.SFX_PICKUP_ITEM" 1.0 1.0 0.0 null null)
  (switch `ETool` (`self.ToolType`)
    (:`RADAR`
      (bind _returnvalue_2 (`|CreateWidget` "/Game/WBP/WBP_InteractPrompt.WBP_InteractPrompt_C" null "Q" "Equip Radar" 2))
      (`UserWidget.AddToViewport` _returnvalue_2 0)
      (add `ToolManager.OnSwitchedToRadar` _returnvalue (delegate `OnSwitchedToRadar_Event`)))
    (:`HEAT_VISION`
      (bind _returnvalue_3 (`|CreateWidget` "/Game/WBP/WBP_InteractPrompt.WBP_InteractPrompt_C" null "E" "Equip Heat Visor" 2))
      (`UserWidget.AddToViewport` _returnvalue_3 0)
      (add `ToolManager.OnSwitchedToHeatVision` _returnvalue (delegate `OnSwitchedToHeatVision_Event`)))
    (:`EMP`
      (bind _returnvalue_4 (`|CreateWidget` "/Game/WBP/WBP_InteractPrompt.WBP_InteractPrompt_C" null "R" "Equip EMP" 2))
      (`UserWidget.AddToViewport` _returnvalue_4 0)
      (add `ToolManager.OnSwitchedToEmp` _returnvalue (delegate `OnSwitchedToEmp_Event`))))
  (`self.SetActorHiddenInGame` true)
  (`self.SetActorEnableCollision` false))

(event `OnSwitchedToHeatVision_Event`
  (`/Engine/EditorBlueprintResources/StandardMacros.IsValid` (stale `self.InteractEventFunction` _returnvalue_3)
    (:`Is Valid`
      (`Widget.RemoveFromParent` (stale `self.InteractEventFunction` _returnvalue_3))
      (goto _label))))

(event `OnSwitchedToEmp_Event`
  (`/Engine/EditorBlueprintResources/StandardMacros.IsValid` (stale `self.InteractEventFunction` _returnvalue_4)
    (:`Is Valid`
      (`Widget.RemoveFromParent` (stale `self.InteractEventFunction` _returnvalue_4))
      (goto _label))))

(event `self.ReceiveBeginPlay`
  (`parent.ReceiveBeginPlay`)
  (cast `/Game/BP/BP_InteractableEmpPickUp` self
    (:`then`
      (set `self.ToolType` "EMP"))
    (:`CastFailed`
      (cast `/Game/BP/BP_InteractableRadarPickUp1` self
        (:`then`
          (set `self.ToolType` "RADAR"))
        (:`CastFailed`
          (cast `/Game/BP/BP_InteractableHeatVisionPickUp2` self)
          (set `self.ToolType` "HEAT_VISION")))))
  (bind _asgame_manager (cast `GameManager` (`GameplayStatics.GetGameInstance`)))
  (add `GameManager.OnSaveDataLoaded` _asgame_manager (delegate `OnSaveDataLoaded_Event`)))

(event `OnSaveDataLoaded_Event`
  (params (SaveGame :type "GP3SaveGame Object Reference"))
  (if (`KismetArrayLibrary.Array_Contains` (`GP3SaveGame.UnlockedTools` SaveGame) (`self.ToolType`))
    (`self.K2_DestroyActor`)))

(fn `UserConstructionScript`
  (`parent.UserConstructionScript`))